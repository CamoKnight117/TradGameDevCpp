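; BP_TileGenerator is an actor that spawns a fixed set of 2,458 BP_generatedWorldTile actors when play begins.
; It stores each tile in TileArray, and a following loop sets InstantiatedMesh to None on indexed tiles.
; Mesh assignment looks unfinished: nodes that build numbered pPlatonic tile mesh names and a debug print are left disconnected.
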(event EventBeginPlay
  (bind _output_get (Variables|Default|SettotalTiles 2458))
  (for _index (range 1 _output_get)
    (bind _returnvalue (Game|SpawnActorfromClass :Class "/Game/MotherEarth/Models/BP_generatedWorldTile.BP_generatedWorldTile_C" :CollisionHandlingOverride "Undefined" :Instigator 0))
    (Utilities|Array|SetArrayElem (Variables|Default|GettileArray) (- _index 1) _returnvalue))
  (for (_ _array_index) 0
    (Variables|/Game/MotherEarth/Models/BP_generatedWorldTile.BP_generatedWorldTile_C|SetinstantiatedMesh (Utilities|Array|Get(acopy) (Variables|Default|GettileArray) _array_index) 0)))

(fn ConstructionScript)