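; One-shot trigger actor that stages the first meteor strike when the player character overlaps it, then destroys itself 30 seconds later.
; It spawns BP_Meteor out along the world-origin-to-strike-point direction at SpawnRadius, facing the origin, and temporarily hands camera focus to it through the player controller.
; The meteor receives this actor and the strike point; SpawnMeteorEnemy, not called here, spawns a gorilla enemy and calls SetGravity with a zero vector.
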(event Custom|CustomEvent_0
  (Actor|DestroyActor))

(event EventBeginPlay)

(event Collision|EventActorBeginOverlap
  (params (OtherActor :type Actor%20Object%20Reference))
  (Utilities|Casting|CastToGravityPlayerCharacter_BP OtherActor)
  (if (Variables|Default|GetfirstTimeActivated)
    (Variables|Default|SetfirstTimeActivated false)
    (CallFunction|SpawnMeteor)
    (Utilities|Time|SetTimerbyEvent (delegate Custom|CustomEvent_0) 3e+01)))

(event EventTick
  (params (DeltaSeconds :type Float%20%28single-precision%29)))

(fn ConstructionScript)

(fn SpawnMeteor
  (bind _spawnradius (Variables|Default|GetspawnRadius))
  (bind _meteorstrikepoint (Variables|Default|GetmeteorStrikePoint))
  (bind _returnvalue (Transformation|GetWorldLocation _meteorstrikepoint))
  (bind _returnvalue_2 (Math|Vector|Normalize _returnvalue))
  (bind _returnvalue_3 (* _returnvalue_2 _spawnradius))
  (bind _returnvalue_4 (Game|SpawnActorfromClass "/Game/MotherEarth/Model_BP/BP_Meteor.BP_Meteor_C" (Math|Transform|MakeTransform _returnvalue_3 (Math|Rotator|FindLookatRotation _returnvalue_3 (Math|Vector|VectorZero)) "1.000000,1.000000,1.000000") "Undefined" 0 0))
  (Variables|/Game/MotherEarth/Model_BP/BP_Meteor.BP_Meteor_C|SetmeteorOwnerFirst _returnvalue_4 self)
  (Variables|/Game/MotherEarth/Model_BP/BP_Meteor.BP_Meteor_C|SetenemySpawnPoint _returnvalue_4 (Variables|Default|GetmeteorStrikePoint))
  (bind _asgravity_player_controller_bp (Utilities|Casting|CastToGravityPlayerController_BP (Game|GetPlayerController 0)))
  (Default|ChangeCameraControl _asgravity_player_controller_bp (Game|Player|GetPlayerPawn 0) _returnvalue_4 (Variables|Default|GetCameraDelayStart) (Variables|Default|GetCameraViewTime) (Variables|Default|GetBlendTime)))

(fn SpawnMeteorEnemy
  (params (spawnLocation :type Capsule%20Component%20Object%20Reference))
  (bind _returnvalue (Game|SpawnActorfromClass "/Game/MotherEarth/AI/Enemy/GravityEnemyGorilla_BP.GravityEnemyGorilla_BP_C" (Transformation|GetWorldTransform spawnLocation) "AlwaysSpawn" 0 0))
  (Default|SetGravity _returnvalue "0, 0, 0"))