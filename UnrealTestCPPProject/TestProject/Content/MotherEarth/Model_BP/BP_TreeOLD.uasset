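; BP_TreeOLD is a tree actor in MotherEarth that grows in stages over time.
; BeginPlay initializes the counters and starts a looping one-second timer that drives the treeTick event.
; Each time the tick count reaches the level-up threshold, the actor's scale is multiplied up and the count resets, until the level-up cap is reached.
; HitPoints is initialized but never used, and the construction script is empty.
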(event Custom|treeTick
  (bind _output_get (Variables|Default|Setcounter (+ (Variables|Default|Getcounter) 1)))
  (if (>= _output_get (Variables|Default|GetlevelUpThreshold))
    (if (< (Variables|Default|GettotalLevelUps) (Variables|Default|GetmaxLevelUps))
      (Transformation|SetActorScale3D (* (Transformation|GetActorScale3D) "1.200000,1.200000,1.200000"))
      (Variables|Default|Setcounter 0)
      (Variables|Default|SettotalLevelUps (+ (Variables|Default|GettotalLevelUps) 1)))))

(event EventBeginPlay
  (Variables|Default|SetHitPoints 0)
  (Variables|Default|Setcounter 0)
  (Variables|Default|SetlevelUpThreshold 5)
  (Variables|Default|SettotalLevelUps 0)
  (Variables|Default|SetmaxLevelUps 2)
  (Utilities|Time|SetTimerbyEvent (delegate Custom|treeTick) 1.0 true))

(fn ConstructionScript)