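; BP_Flower is a flower actor that tracks player and minion characters standing in it and can die.
; While alive, overlap begin adds to the character's flower overlap count, and overlap end always removes from it.
; SetDead hides the mesh, briefly plays death particles, then, if a TileOwner is valid, deregisters from that tile and destroys itself after a delay.
; SetAlive restores the alive flag and stops particles, leaving mesh visibility untouched.
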(event Collision|EventActorBeginOverlap
  (params (OtherActor :type Actor%20Object%20Reference))
  (if (Variables|Default|Getalive)
    (bind _asgravity_player_character_bp (Utilities|Casting|CastToGravityPlayerCharacter_BP OtherActor)
      (:then
        (Default|AddtoFlowerOverlap _asgravity_player_character_bp))
      (:CastFailed
        (bind _asgravity_minion_character_bp (Utilities|Casting|CastToGravityMinionCharacter_BP OtherActor))
        (Default|AddtoFlowerOverlap _asgravity_minion_character_bp)))))

(event Collision|EventActorEndOverlap
  (params (OtherActor :type Actor%20Object%20Reference))
  (bind _asgravity_player_character_bp (Utilities|Casting|CastToGravityPlayerCharacter_BP OtherActor)
    (:then
      (Default|RemovefromFlowerOverlap _asgravity_player_character_bp))
    (:CastFailed
      (bind _asgravity_minion_character_bp (Utilities|Casting|CastToGravityMinionCharacter_BP OtherActor))
      (Default|RemovefromFlowerOverlap _asgravity_minion_character_bp))))

(fn ConstructionScript)

(fn SetDead
  (bind _tileowner (Variables|Default|GettileOwner))
  (Variables|Default|Setalive false)
  (Components|Activation|Activate (Variables|Default|GetdeadFlowerParticles) false)
  (Rendering|SetVisibility (Variables|Default|GetStaticMesh) false false)
  (Utilities|Time|SetTimerbyFunctionName 0 "deactivateParticles" 0.5)
  (Utilities|IsValid _tileowner
    (:Is%20Valid
      (Utilities|Set|Remove (Variables|/Game/MotherEarth/WorldTileChild.WorldTileChild_C|GetflowerObjects _tileowner) self)
      (Math|Integer|DecrementInt (Variables|/Game/MotherEarth/WorldTileChild.WorldTileChild_C|GetNumSmallPlants _tileowner)
        (:%20%20
          (Utilities|Time|SetTimerbyFunctionName 0 "destroySelf" 3.0))))))

(fn SetAlive
  (Variables|Default|Setalive true)
  (Components|Activation|Deactivate (Variables|Default|GetdeadFlowerParticles)))

(fn DestroySelf
  (Actor|DestroyActor))

(fn DeactivateParticles
  (Components|Activation|Deactivate (Variables|Default|GetdeadFlowerParticles)))