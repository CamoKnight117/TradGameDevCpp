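; BP_PillarMarkerFlowers is a pillar marker that shows its state with three effect systems: blue when deactivated, green when activated, red when taken by an enemy.
; It starts deactivated at BeginPlay, and each state function turns on its own system and stops the other two; the enemy state only applies if CanBeEnemy is set.
; The first activation also starts a linked MovableMountain, or a MovableBridge if no valid mountain is set.
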(event EventBeginPlay
  (CallFunction|Deactivate))

(fn ConstructionScript)

(fn Activate
  (bind _movablemountain (Variables|Default|GetmovableMountain))
  (bind _movablebridge (Variables|Default|GetmovableBridge))
  (Development|PrintString "activated")
  (Components|Activation|Activate (Variables|Default|GetgreenSystem) false)
  (Components|Activation|Deactivate (Variables|Default|GetredSystem))
  (Components|Activation|Deactivate (Variables|Default|GetblueSystem))
  (if (not (Variables|Default|GetpreviouslyActivated))
    (Variables|Default|SetpreviouslyActivated true)
    (Utilities|IsValid _movablemountain
      (:Is%20Valid
        (Default|StartMountainActivation _movablemountain true))
      (:Is%20Not%20Valid
        (Utilities|IsValid _movablebridge
          (:Is%20Valid
            (Default|StartBridgeActivation _movablebridge true)))))))

(fn Deactivate
  (Components|Activation|Activate (Variables|Default|GetblueSystem) false)
  (Components|Activation|Deactivate (Variables|Default|GetgreenSystem))
  (Components|Activation|Deactivate (Variables|Default|GetredSystem)))

(fn EnemyActivate
  (if (Variables|Default|GetcanBeEnemy)
    (Components|Activation|Activate (Variables|Default|GetredSystem) false)
    (Components|Activation|Deactivate (Variables|Default|GetblueSystem))
    (Components|Activation|Deactivate (Variables|Default|GetgreenSystem))))