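; Carnivore plant minion, an allied defender that spits BP_CarnivoreSpit projectiles at the nearest listed enemy on a tick-counted cooldown.
; EnemyList fills only from TargetSphere overlaps at BeginPlay; the delayed sphere sweep feeds no live add or remove logic.
; AttackZone overlaps start and stop enemy attacks on the plant.
; Damage and timed self-healing drive a camera-facing health bar; death notifies the owning WorldTileChild and destroys the actor.
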(event OnComponentBeginOverlap(AttackZone)
  (params (OverlappedComponent :type Primitive%20Component%20Object%20Reference) (OtherActor :type Actor%20Object%20Reference) (OtherComp :type Primitive%20Component%20Object%20Reference) (OtherBodyIndex :type Integer) (bFromSweep :type Boolean) (SweepResult :type Hit%20Result%20Structure%20%28by%20ref%29))
  ;[1 1 1] Custom code for enemy attacks so they ignore the TargetSphere
  (bind _asgravity_enemy_character_bp (Utilities|Casting|CastToGravityEnemyCharacter_BP OtherActor))
  (Default|AttackPlant _asgravity_enemy_character_bp self))

(event OnComponentEndOverlap(AttackZone)
  (params (OverlappedComponent :type Primitive%20Component%20Object%20Reference) (OtherActor :type Actor%20Object%20Reference) (OtherComp :type Primitive%20Component%20Object%20Reference) (OtherBodyIndex :type Integer))
  ;[1 1 1] Custom code for enemy attacks so they ignore the TargetSphere
  (bind _asgravity_enemy_character_bp (Utilities|Casting|CastToGravityEnemyCharacter_BP OtherActor))
  (Default|EndAttackPlant _asgravity_enemy_character_bp self))

(event Custom|OnTakeAnyDamage_Event
  (params (DamagedActor :type Actor%20Object%20Reference) (Damage :type Float%20%28single-precision%29) (DamageType :type Damage%20Type%20Object%20Reference) (InstigatedBy :type Controller%20Object%20Reference) (DamageCauser :type Actor%20Object%20Reference))
  ;[1 1 1] If damaged, decrease CurrentHealth and update the health bar, and destroy the actor if health less than 0
  (Rendering|SetVisibility (Variables|Default|GetHealthBar) true false)
  (bind _output_get (Variables|Default|SetCurrentHealth (- (Variables|Default|GetCurrentHealth) Damage)))
  (bind _asbp_ally_health_bar (Utilities|Casting|CastToBP_AllyHealthBar (UserInterface|GetWidget (Variables|Default|GetHealthBar))))
  (Default|SetHealth _asbp_ally_health_bar (/ _output_get (Variables|Default|GetTotalHealth)))
  (if (<= (Variables|Default|GetCurrentHealth) 0.0)
    (bind _asworld_tile_child (Utilities|Casting|CastToWorldTileChild (Components|GetOwner))
      (:then
        (Default|OnTreeDestroyed _asworld_tile_child))
      (:CastFailed
        _))
    (Actor|DestroyActor)))

(event Custom|sweepBack
  ;[1 1 1] Move the collision sphere away, then back to trigger begin overlap events
  (Transformation|SetRelativeLocation (Variables|Default|GettargetSphere) "0, 0, 0" true false))

(event Custom|OnHealDamage
  (params (RestoredHealth :type Float%20%28double-precision%29))
  (bind _healthbar (Variables|Default|GetHealthBar))
  ;[1 1 1] If healed, increase CurrentHealth and update the health bar, with max possible health being equal to TotalHealth
  (if (<= (+ RestoredHealth (Variables|Default|GetCurrentHealth)) (Variables|Default|GetTotalHealth))
    (Variables|Default|SetCurrentHealth (+ RestoredHealth (Variables|Default|GetCurrentHealth)))
    (else
      (Variables|Default|SetCurrentHealth (Variables|Default|GetTotalHealth))
      (Rendering|SetVisibility _healthbar false false)))
  (bind _asbp_ally_health_bar (Utilities|Casting|CastToBP_AllyHealthBar (UserInterface|GetWidget _healthbar)))
  (Default|SetHealth _asbp_ally_health_bar (/ (Variables|Default|GetCurrentHealth) (Variables|Default|GetTotalHealth))))

(event EventTick
  (params (DeltaSeconds :type Float%20%28single-precision%29))
  (bind _returnvalue (Game|GetPlayerCameraManager 0))
  (bind _healthbar (Variables|Default|GetHealthBar))
  (if (< (Variables|Default|GetattackCooldownCounter) (Variables|Default|GetattackCooldownMax))
    (Math|Integer|IncrementInt (Variables|Default|GetattackCooldownCounter)
      (:%20%20
        _)))
  ;[1 1 1] Keep the health bar rotated so the player can see it
  (Transformation|SetWorldRotation _healthbar (Math|Rotator|FindLookatRotation (Transformation|GetActorLocation (Game|Player|GetPlayerPawn 0)) (Camera|GetCameraLocation _returnvalue)) false false)
  (Transformation|AddRelativeRotation _healthbar (Class|KismetMathLibrary|NegateRotator (Math|Rotator|MakeRotator (.Roll (Math|Rotator|BreakRotator (Camera|GetCameraRotation _returnvalue))) 0.0 0.0)) false false)
  (if (== (Variables|Default|GetattackCooldownCounter) (Variables|Default|GetattackCooldownMax))
    (if (> (Utilities|Array|Length (Variables|Default|GetenemyList)) 0)
      (CallFunction|FireProjectile (Transformation|GetActorLocation (.ReturnValue (Actor|FindNearestActor (Transformation|GetWorldLocation (Variables|Default|GetDefaultSceneRoot)) (Variables|Default|GetenemyList)))))
      (Variables|Default|SetattackCooldownCounter 0))))

(event EventBeginPlay
  ;[1 1 1] Add overlapping enemies to enemy list
  (for _array_element (Collision|GetOverlappingActors (Variables|Default|GettargetSphere) "/Game/MotherEarth/AI/Enemy/GravityEnemyCharacter_BP.GravityEnemyCharacter_BP_C" :!class /Script/Engine.PrimitiveComponent)
    (bind _asgravity_enemy_character_bp (Utilities|Casting|CastToGravityEnemyCharacter_BP _array_element))
    (Utilities|Array|Add (Variables|Default|GetenemyList) _asgravity_enemy_character_bp))
  (Utilities|Time|SetTimerbyFunctionName 0 "healOverTime" 3.0)
  (Rendering|SetVisibility (Variables|Default|GetHealthBar) false false)
  ;[1 1 1] If damaged, decrease CurrentHealth and update the health bar, and destroy the actor if health less than 0
  (EventDispatchers|BindEventtoOnTakeAnyDamage (delegate Custom|OnTakeAnyDamage_Event))
  (Variables|Default|SetCurrentHealth (Variables|Default|GetTotalHealth))
  ;[1 1 1] Move the collision sphere away, then back to trigger begin overlap events
  (Transformation|SetRelativeLocation (Variables|Default|GettargetSphere) (* (Transformation|GetActorLocation) 5.0) false true)
  (Utilities|Time|SetTimerbyEvent (delegate Custom|sweepBack) 1.0))

(event Collision|EventActorBeginOverlap
  (params (OtherActor :type Actor%20Object%20Reference)))

(event Collision|EventActorEndOverlap
  (params (OtherActor :type Actor%20Object%20Reference)))

(fn ConstructionScript)

(fn HealOverTime
  (Utilities|IsValid self
    (:Is%20Valid
      (Utilities|Time|SetTimerbyFunctionName 0 "healOverTime" 3.0)
      (CallFunction|OnHealDamage (Variables|Default|GetHealRate)))))

(fn FireProjectile
  (params (targetLocation :type Vector))
  (bind _spitspawn (Variables|Default|GetspitSpawn))
  (bind _returnvalue (Transformation|GetWorldLocation _spitspawn))
  (Game|SpawnActorfromClass "/Game/MotherEarth/Model_BP/BP_CarnivoreSpit.BP_CarnivoreSpit_C" (Math|Transform|MakeTransform _returnvalue (Math|Rotator|FindLookatRotation _returnvalue targetLocation) "1.000000,1.000000,1.000000") "Undefined" 0 0))