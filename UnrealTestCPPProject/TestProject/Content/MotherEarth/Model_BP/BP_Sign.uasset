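; BP_Sign is a world sign that shows a message on static and floating text widgets, the latter toggled as the player enters or leaves its overlap.
; BeginPlay copies MessageText into both widgets.
; Each Tick turns the floating text along the player-pawn-to-camera direction and counters camera roll so it faces the view.
; PlayerOverlapping is set true on both overlap begin and end, and is not read here.
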(event EventTick
  (params (DeltaSeconds :type Float%20%28single-precision%29))
  (bind _returnvalue (Game|GetPlayerCameraManager 0))
  (bind _floatingtext (Variables|Default|GetFloatingText))
  ;[1 1 1] Keep the radial rotated so the player can see it
  (if true
    (Transformation|SetWorldRotation _floatingtext (Math|Rotator|FindLookatRotation (Transformation|GetActorLocation (Game|Player|GetPlayerPawn 0)) (Camera|GetCameraLocation _returnvalue)) false false)
    (Transformation|AddRelativeRotation _floatingtext (Class|KismetMathLibrary|NegateRotator (Math|Rotator|MakeRotator (.Roll (Math|Rotator|BreakRotator (Camera|GetCameraRotation _returnvalue))) 0.0 0.0)) false false)))

(event EventBeginPlay
  (bind _asbp_sign_message (Utilities|Casting|CastToBP_SignMessage (UserInterface|GetWidget (Variables|Default|GetFloatingText))))
  (Variables|/Game/MotherEarth/UI/BP_SignMessage.BP_SignMessage_C|SetmessageText _asbp_sign_message (Variables|Default|GetmessageText))
  (bind _asbp_sign_static_message (Utilities|Casting|CastToBP_SignStaticMessage (UserInterface|GetWidget (Variables|Default|GetStaticText))))
  (Variables|/Game/MotherEarth/UI/BP_SignStaticMessage.BP_SignStaticMessage_C|SetmessageText _asbp_sign_static_message (Variables|Default|GetmessageText)))

(event Collision|EventActorBeginOverlap
  (params (OtherActor :type Actor%20Object%20Reference))
  (Utilities|Casting|CastToGravityPlayerCharacter_BP OtherActor)
  (Variables|Default|SetplayerOverlapping true)
  (Rendering|SetVisibility (Variables|Default|GetFloatingText) true false))

(event Collision|EventActorEndOverlap
  (params (OtherActor :type Actor%20Object%20Reference))
  (Utilities|Casting|CastToGravityPlayerCharacter_BP OtherActor)
  (Variables|Default|SetplayerOverlapping true)
  (Rendering|SetVisibility (Variables|Default|GetFloatingText) false false))

(fn ConstructionScript)