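; BP_WorldTile_Parent is a world tile that turns to grass when the gravity player character walks on it and can then grow trees.
; Clicking a grass tile without Left Shift held calls SpawnTree, which allows three trees at fixed tile-relative offsets.
; A temporary BP_SpawnCube tests each spot for player overlap before the tree spawns, then is destroyed.
; The prototype random spawning at start is disconnected.
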(event EventBeginPlay
  ;[1 1 1] Spawn trees randomly at start (prototype use only)
)

(event Collision|EventActorBeginOverlap
  (params (OtherActor :type Actor%20Object%20Reference))
  ;[1 1 1] Turn walked on tiles into grass
  (Utilities|Casting|CastToGravityPlayerCharacter_BP OtherActor)
  (Rendering|Material|SetMaterial (Variables|Default|GetCube) 0 "/Game/MotherEarth/Materials/MAT_greenGrass.MAT_greenGrass")
  (Variables|Default|SetIsGrass true))

(event MouseInput|EventActorOnClicked
  (params (ButtonPressed :type Key%20Structure :default "None"))
  ;[1 1 1] Spawn a tree if grass tile clicked
  (if (Variables|Default|GetIsGrass)
    (bind _asgravity_player_controller_bp (Utilities|Casting|CastToGravityPlayerController_BP (Game|GetPlayerController 0)))
    (if (not (Variables|/Game/MotherEarth/GameObjects/GravityPlayerController_BP.GravityPlayerController_BP_C|GetleftShiftPressed _asgravity_player_controller_bp))
      (CallFunction|SpawnTree))))

(fn ConstructionScript)

(fn SpawnTree
  (bind _returnvalue (Transformation|GetActorRotation))
  (bind _returnvalue_2 (Transformation|GetActorLocation))
  (bind _numtrees (Variables|Default|GetNumTrees))
  (bind _returnvalue_3 (Math|Transform|MakeTransform _returnvalue_2 _returnvalue))
  ;[1 1 1] Set each tree to have different position - 3 trees max
  (if (< _numtrees 3)
    (switch int _numtrees
      (:0
        (Variables|Default|SetTreeOffset "150.000000,0.000000,0.000000"))
      (:1
        (Variables|Default|SetTreeOffset "-40.000000,100.000000,0.000000"))
      (:2
        (Variables|Default|SetTreeOffset "-200.000000,-75.000000,0.000000")))
    ;[1 1 1] Use spawn cube to determine if player is overlapping tree spawning location
    (bind _returnvalue_4 (Game|SpawnActorfromClass "/Game/MotherEarth/Model_BP/BP_SpawnCube.BP_SpawnCube_C" _returnvalue_3 "AlwaysSpawn" 0 0))
    (bind _output_get (Variables|Default|SetCurrSpawnCube _returnvalue_4))
    (Transformation|AddRelativeLocation (Variables|/Game/MotherEarth/Model_BP/BP_SpawnCube.BP_SpawnCube_C|GetBase _output_get) (Variables|Default|GetTreeOffset) false true)
    (if (Collision|IsOverlappingActor (Variables|Default|GetCurrSpawnCube) (Game|GetPlayerCharacter 0) :!class /Script/Engine.Actor)
      _
      (else
        ;[1 1 1] Spawn tree and move to relative location  if able and then increment tree count. Always delete spawn cube
        (bind _returnvalue_5 (Game|SpawnActorfromClass "/Game/MotherEarth/Model_BP/BP_Tree.BP_Tree_C" _returnvalue_3 "AlwaysSpawn" 0 0))
        (Transformation|AddRelativeLocation (Variables|/Game/MotherEarth/Model_BP/BP_Tree.BP_Tree_C|GetBase _returnvalue_5) (Variables|Default|GetTreeOffset) false true)
        (Math|Integer|IncrementInt (Variables|Default|GetNumTrees)
          (:%20%20
            _))))
    (Actor|DestroyActor (Variables|Default|GetCurrSpawnCube))))