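; BP_PillarMarkerGrass is a pillar marker with three states shown by toggling green, red and white effect systems, starting in the white deactivated state.
; EnemyActivate switches it to red, while Activate switches it to green.
; On first activation only, it sets timers to call SinkWall on a linked MovableMountain and SummonBridge on a linked MovableBridge, if valid, and has GravityPlayerController_BP shift the camera view to each.
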(event EventBeginPlay
  (CallFunction|Deactivate))

(event Collision|EventActorBeginOverlap
  (params (OtherActor :type Actor%20Object%20Reference)))

(event EventTick
  (params (DeltaSeconds :type Float%20%28single-precision%29)))

(fn ConstructionScript)

(fn Activate
  (bind _movablemountain (Variables|Default|GetmovableMountain))
  (bind _movablebridge (Variables|Default|GetmovableBridge))
  (Components|Activation|Activate (Variables|Default|GetgreenSystem) false)
  (Components|Activation|Deactivate (Variables|Default|GetredSystem))
  (Components|Activation|Deactivate (Variables|Default|GetwhiteSystem))
  (if (not (Variables|Default|GetpreviouslyActivated))
    (Variables|Default|SetpreviouslyActivated true)
    (Utilities|IsValid _movablemountain
      (:Is%20Valid
        (Utilities|Time|SetTimerbyFunctionName _movablemountain "SinkWall" 3.0)
        (bind _asgravity_player_controller_bp (Utilities|Casting|CastToGravityPlayerController_BP (Game|GetPlayerController 0)))
        (Default|ChangeCameraControl _asgravity_player_controller_bp (Game|Player|GetPlayerPawn 0) (Variables|Default|GetmovableMountain) 2.0 8.0 1.0))
      (:Is%20Not%20Valid
        _))
    (Utilities|IsValid _movablebridge
      (:Is%20Valid
        (Utilities|Time|SetTimerbyFunctionName _movablebridge "SummonBridge" 1.0)
        (bind _asgravity_player_controller_bp_2 (Utilities|Casting|CastToGravityPlayerController_BP (Game|GetPlayerController 0)))
        (Default|ChangeCameraControl _asgravity_player_controller_bp_2 (Game|Player|GetPlayerPawn 0) (Variables|Default|GetmovableBridge) 2.0 8.0 1.0)))))

(fn Deactivate
  (Components|Activation|Activate (Variables|Default|GetwhiteSystem) false)
  (Components|Activation|Deactivate (Variables|Default|GetgreenSystem))
  (Components|Activation|Deactivate (Variables|Default|GetredSystem)))

(fn EnemyActivate
  (Components|Activation|Activate (Variables|Default|GetredSystem) false)
  (Components|Activation|Deactivate (Variables|Default|GetwhiteSystem))
  (Components|Activation|Deactivate (Variables|Default|GetgreenSystem)))