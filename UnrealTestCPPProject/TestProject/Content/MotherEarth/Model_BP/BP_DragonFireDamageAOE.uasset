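; One-shot dragon fire area-of-effect actor that damages players, gravity minions and carnivore minions, then destroys itself.
; On BeginPlay it teleports its collision sphere away and shortly sweeps it back to the actor's origin to force begin-overlap events.
; Overlap begin and end events maintain a list of those three character types.
; A short timer after the sweep applies fixed damage to everyone listed and destroys the actor.
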(event Custom|DamageAndDestroy
  (for _array_element (Variables|Default|GetactorsToDamage)
    (Game|Damage|ApplyDamage _array_element 3e+01 0 0))
  (Actor|DestroyActor))

(event Custom|sweepBack
  ;[1 1 1] Move the collision sphere away, then back to trigger begin overlap events
  (Transformation|SetRelativeLocation (Variables|Default|GetSphere) "0, 0, 0" true false)
  (Utilities|Time|SetTimerbyEvent (delegate Custom|DamageAndDestroy) 0.1))

(event EventBeginPlay
  ;[1 1 1] Move the collision sphere away, then back to trigger begin overlap events
  (Transformation|SetRelativeLocation (Variables|Default|GetSphere) (* (Transformation|GetActorLocation) 5.0) false true)
  (Utilities|Time|SetTimerbyEvent (delegate Custom|sweepBack) 0.1))

(event Collision|EventActorBeginOverlap
  (params (OtherActor :type Actor%20Object%20Reference))
  (Utilities|Casting|CastToGravityPlayerCharacter_BP OtherActor
    (:then
      _)
    (:CastFailed
      (Utilities|Casting|CastToGravityMinionCharacter_BP OtherActor
        (:then
          _)
        (:CastFailed
          (Utilities|Casting|CastToBP_CarnivoreMinion OtherActor)))))
  (Utilities|Array|Add (Variables|Default|GetactorsToDamage) OtherActor))

(event Collision|EventActorEndOverlap
  (params (OtherActor :type Actor%20Object%20Reference))
  (Utilities|Casting|CastToGravityPlayerCharacter_BP OtherActor
    (:then
      _)
    (:CastFailed
      (Utilities|Casting|CastToGravityMinionCharacter_BP OtherActor
        (:then
          _)
        (:CastFailed
          (Utilities|Casting|CastToBP_CarnivoreMinion OtherActor)))))
  (Utilities|Array|RemoveItem (Variables|Default|GetactorsToDamage) OtherActor))

(fn ConstructionScript)