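; BP_Meteor is a meteor that sheds debris and, on impact with a land or water world tile, spawns an enemy.
; Tick counts frames and spawns a BP_MeteorChunk2 whenever a threshold, re-randomized around ChunkThreshold, is passed.
; On overlap it bursts into BP_MeteorChunk actors aimed in a random cone around its direction from world origin.
; It then asks MeteorOwner to spawn the enemy at EnemySpawnPoint and destroys itself.
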(event EventBeginPlay
  (bind _chunkthreshold (Variables|Default|GetchunkThreshold))
  (bind _returnvalue (/ _chunkthreshold 2))
  (Variables|Default|SetchunkThresholdRandomized (Math|Random|RandomIntegerinRange (- _chunkthreshold _returnvalue) (+ _chunkthreshold _returnvalue))))

(event EventTick
  (params (DeltaSeconds :type Float%20%28single-precision%29))
  (bind _returnvalue (Transformation|GetActorLocation))
  (bind _chunkthreshold (Variables|Default|GetchunkThreshold))
  (bind _returnvalue_2 (/ _chunkthreshold 2))
  (Math|Integer|IncrementInt (Variables|Default|Getcount)
    (:%20%20
      (if (> (Variables|Default|Getcount) (Variables|Default|GetchunkThresholdRandomized))
        (Game|SpawnActorfromClass "/Game/MotherEarth/Model_BP/BP_MeteorChunk2.BP_MeteorChunk2_C" (Math|Transform|MakeTransform _returnvalue (Math|Rotator|FindLookatRotation _returnvalue (* (Math|Random|RandomUnitVectorinConeinDegrees (Math|Vector|NegateVector _returnvalue) 8e+01) "1000.000000,1000.000000,1000.000000")) "1.000000,1.000000,1.000000") "Undefined" 0 0)
        (Variables|Default|Setcount 0)
        (Variables|Default|SetchunkThresholdRandomized (Math|Random|RandomIntegerinRange (- _chunkthreshold _returnvalue_2) (+ _chunkthreshold _returnvalue_2)))))))

(event Collision|EventActorBeginOverlap
  (params (OtherActor :type Actor%20Object%20Reference))
  (bind _returnvalue (Transformation|GetActorLocation))
  (Utilities|Casting|CastToWorldTileChild OtherActor
    (:then
      _)
    (:CastFailed
      (Utilities|Casting|CastToWorldWaterTileChild OtherActor)))
  (for _index (range 0 10)
    (Game|SpawnActorfromClass "/Game/MotherEarth/Model_BP/BP_MeteorChunk.BP_MeteorChunk_C" (Math|Transform|MakeTransform _returnvalue (Math|Rotator|FindLookatRotation (Math|Vector|VectorZero) (* (Math|Random|RandomUnitVectorinConeinDegrees _returnvalue 85.0) "1000.000000,1000.000000,1000.000000")) "1.000000,1.000000,1.000000") "Undefined" 0 0))
  (Default|SpawnMeteorEnemy (Variables|Default|GetmeteorOwner) (Variables|Default|GetenemySpawnPoint))
  (Actor|DestroyActor))

(fn ConstructionScript)