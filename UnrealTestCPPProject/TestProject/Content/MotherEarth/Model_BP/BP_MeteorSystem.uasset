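; Meteor shower spawner that periodically launches BP_Meteor actors around the world origin, which they face on spawn.
; Tick counts frames to a threshold, re-randomized within a quarter of MeteorShowerThreshold either way, then spawns a meteor at SpawnRadius along one of six spawn components' directions.
; Each meteor receives this system and that component; SpawnMeteorEnemy, not called here, spawns a gravity enemy at a supplied component.
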(event EventBeginPlay
  (bind _meteorshowerthreshold (Variables|Default|GetmeteorShowerThreshold))
  (bind _returnvalue (/ _meteorshowerthreshold 4))
  (Variables|Default|SetmeteorThresholdRandomized (Math|Random|RandomIntegerinRange (- _meteorshowerthreshold _returnvalue) (+ _meteorshowerthreshold _returnvalue))))

(event EventTick
  (params (DeltaSeconds :type Float%20%28single-precision%29))
  (bind _meteorshowerthreshold (Variables|Default|GetmeteorShowerThreshold))
  (bind _returnvalue (/ _meteorshowerthreshold 4))
  (bind _result (Math|Integer|IncrementInt (Variables|Default|GetmeteorCount))
    (:%20%20
      (if (> _result (Variables|Default|GetmeteorThresholdRandomized))
        (Variables|Default|SetmeteorThresholdRandomized (Math|Random|RandomIntegerinRange (- _meteorshowerthreshold _returnvalue) (+ _meteorshowerthreshold _returnvalue)))
        (CallFunction|SpawnMeteor)))))

(fn ConstructionScript)

(fn SpawnMeteor
  (bind _spawnlocation (CallFunction|GetRandomSpawnComponent))
  (bind _returnvalue (Game|SpawnActorfromClass "/Game/MotherEarth/Model_BP/BP_Meteor.BP_Meteor_C" (Math|Transform|MakeTransform (* (Math|Vector|Normalize (Transformation|GetWorldLocation _spawnlocation)) (Variables|Default|GetspawnRadius)) (Math|Rotator|FindLookatRotation (* (Math|Vector|Normalize (Transformation|GetWorldLocation _spawnlocation)) (Variables|Default|GetspawnRadius)) (Math|Vector|VectorZero)) "1.000000,1.000000,1.000000") "Undefined" 0 0))
  (Variables|/Game/MotherEarth/Model_BP/BP_Meteor.BP_Meteor_C|SetmeteorOwner _returnvalue self)
  (Variables|/Game/MotherEarth/Model_BP/BP_Meteor.BP_Meteor_C|SetenemySpawnPoint _returnvalue _spawnlocation)
  (Variables|Default|SetmeteorCount 0))

(fn GetRandomSpawnComponent
  (switch int (Math|Random|RandomIntegerinRange 0 5)
    (:Default
      _)
    (:0
      _)
    (:1
      (return (Variables|Default|GetverticalSliceSpawn2)))
    (:2
      (return (Variables|Default|GetverticalSliceSpawn3)))
    (:3
      (return (Variables|Default|GetverticalSliceSpawn4)))
    (:4
      (return (Variables|Default|GetverticalSliceSpawn5)))
    (:5
      (return (Variables|Default|GetverticalSliceSpawn6))))
  (return (Variables|Default|GetverticalSliceSpawn1)))

(fn SpawnMeteorEnemy
  (params (spawnLocation :type Capsule%20Component%20Object%20Reference))
  (bind _returnvalue (Game|SpawnActorfromClass "/Game/MotherEarth/AI/Enemy/GravityEnemyCharacter_BP.GravityEnemyCharacter_BP_C" (Transformation|GetWorldTransform spawnLocation) "AdjustIfPossibleButAlwaysSpawn" 0 0))
  (Default|SetGravity _returnvalue "0, 0, 0"))