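; BP_MovingMountain is a one-shot mountain barrier that, once activated, opens up and sinks toward the world origin.
; Activation starts a delayed sink and can hand the camera to the mountain through GravityPlayerController_BP.
; SinkWall disables collision and destroys both walls, then next-tick timers step the actor inward by StepSize, so speed depends on frame rate.
; The actor destroys itself within a StepSize-scaled distance of the origin.
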(fn ConstructionScript)

(fn SinkWall
  (bind _returnvalue (Transformation|GetActorTransform))
  (bind _scene (Variables|Default|GetScene))
  (bind _returnvalue_2 (Transformation|GetWorldLocation _scene))
  (Collision|SetCollisionEnabled (Variables|Default|Getwall1) "NoCollision")
  (Collision|SetCollisionEnabled (Variables|Default|Getwall2) "NoCollision")
  (Collision|SetCollisionEnabled (Variables|Default|GetMountainShape) "NoCollision")
  (Components|DestroyComponent (Variables|Default|Getwall1))
  (Components|DestroyComponent (Variables|Default|Getwall2))
  (Transformation|SetActorTransform (Math|Transform|MakeTransform (+ _returnvalue_2 (* (- (Math|Vector|VectorZero) _returnvalue_2) (/ (Variables|Default|GetstepSize) (Math|Vector|VectorLength _returnvalue_2)))) (.rotation _returnvalue) (.scale _returnvalue)))
  (if (not (< (Math|Vector|VectorLength (Transformation|GetWorldLocation (Variables|Default|GetScene))) (* (Variables|Default|GetstepSize) 3.0)))
    (Class|KismetSystemLibrary|SetTimerforNextTick 0 "SinkWallRecurse")))

(fn SinkWallRecurse
  (bind _returnvalue (Transformation|GetActorTransform))
  (bind _scene (Variables|Default|GetScene))
  (bind _returnvalue_2 (Transformation|GetWorldLocation _scene))
  (Transformation|SetActorTransform (Math|Transform|MakeTransform (+ _returnvalue_2 (* (- (Math|Vector|VectorZero) _returnvalue_2) (/ (Variables|Default|GetstepSize) (Math|Vector|VectorLength _returnvalue_2)))) (.rotation _returnvalue) (.scale _returnvalue)))
  (if (< (Math|Vector|VectorLength (Transformation|GetWorldLocation (Variables|Default|GetScene))) (* (Variables|Default|GetstepSize) 2.6e+03))
    (Actor|DestroyActor)
    (else
      (Class|KismetSystemLibrary|SetTimerforNextTick 0 "SinkWallRecurse"))))

(fn StartMountainActivation
  (params (UseCameraChange :type Boolean))
  (if (not (Variables|Default|GethasBeenActivatedAlready))
    (Variables|Default|SethasBeenActivatedAlready true)
    (Utilities|Time|SetTimerbyFunctionName 0 "SinkWall" (Variables|Default|GetActivationDelay))
    (bind _asgravity_player_controller_bp (Utilities|Casting|CastToGravityPlayerController_BP (Game|GetPlayerController 0)))
    (if UseCameraChange
      (Default|ChangeCameraControl _asgravity_player_controller_bp (Game|Player|GetPlayerPawn 0) self (Variables|Default|GetCameraDelayStart) (Variables|Default|GetCameraViewTime) (Variables|Default|GetBlendTime)))))