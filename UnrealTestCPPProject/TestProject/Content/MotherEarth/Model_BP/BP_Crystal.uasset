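; BP_Crystal is a destructible enemy spawner that summons its linked bridge and sinks its linked mountain when destroyed.
; Tick counts frames to a randomized threshold, then spawns gravity enemies at five points in rotation, up to SpawnMax, setting itself as their HomeCrystal.
; Damage reveals and updates a camera-facing health bar.
; Ctrl-click release outside marquee selection makes the crystal the target of the player's selected units.
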(event Custom|OnTakeAnyDamage_Event
  (params (DamagedActor :type Actor%20Object%20Reference) (Damage :type Float%20%28single-precision%29) (DamageType :type Damage%20Type%20Object%20Reference) (InstigatedBy :type Controller%20Object%20Reference) (DamageCauser :type Actor%20Object%20Reference))
  (bind _movablebridge (Variables|Default|GetmovableBridge))
  (bind _movablemountain (Variables|Default|GetmovableMountain))
  ;[1 1 1] If damaged, decrease CurrentHealth and update the health bar, and destroy the actor if health less than 0
  (Development|PrintString "Damage")
  (Rendering|SetVisibility (Variables|Default|GetHealthBar) true false)
  (bind _output_get (Variables|Default|SetCurrentHealth (- (Variables|Default|GetCurrentHealth) Damage)))
  (bind _asbp_enemy_health_bar (Utilities|Casting|CastToBP_EnemyHealthBar (UserInterface|GetWidget (Variables|Default|GetHealthBar))))
  (Default|SetHealth _asbp_enemy_health_bar (/ _output_get (Variables|Default|GetTotalHealth)))
  (if (<= (Variables|Default|GetCurrentHealth) 0.0)
    (Utilities|IsValid _movablebridge
      (:Is%20Valid
        (Default|SummonBridge _movablebridge))
      (:Is%20Not%20Valid
        _))
    (Utilities|IsValid _movablemountain
      (:Is%20Valid
        (Default|SinkWall _movablemountain))
      (:Is%20Not%20Valid
        _))
    (Actor|DestroyActor)))

(event EventBeginPlay
  (bind _spawnthreshold (Variables|Default|GetspawnThreshold))
  (bind _spawnpointarray (Variables|Default|GetspawnPointArray))
  (bind _returnvalue (/ _spawnthreshold 4))
  ;[1 1 1] Initial set up
  (Utilities|Array|Add _spawnpointarray (Variables|Default|GetSpawn%20Point%201))
  (Utilities|Array|Add _spawnpointarray (Variables|Default|GetSpawn%20Point%202))
  (Utilities|Array|Add _spawnpointarray (Variables|Default|GetSpawn%20Point%203))
  (Utilities|Array|Add _spawnpointarray (Variables|Default|GetSpawn%20Point%204))
  (Utilities|Array|Add _spawnpointarray (Variables|Default|GetSpawn%20Point%205))
  (Variables|Default|SetrandomizedSpawnThreshold (Math|Random|RandomIntegerinRange (- _spawnthreshold _returnvalue) (+ _spawnthreshold _returnvalue)))
  (Rendering|SetVisibility (Variables|Default|GetHealthBar) false false)
  (EventDispatchers|BindEventtoOnTakeAnyDamage (delegate Custom|OnTakeAnyDamage_Event))
  (Variables|Default|SetCurrentHealth (Variables|Default|GetTotalHealth)))

(event EventActorOnReleased
  (params (ButtonReleased :type Key%20Structure :default "None"))
  ;[1 1 1] Targetting logic
  (bind _asgravity_player_controller_bp (Utilities|Casting|CastToGravityPlayerController_BP (Game|GetPlayerController 0)))
  (if (Variables|/Game/MotherEarth/GameObjects/GravityPlayerController_BP.GravityPlayerController_BP_C|GetleftCtrlPressed _asgravity_player_controller_bp)
    (bind _asme_hud (Utilities|Casting|CastToME_HUD (HUD|GetHUD _asgravity_player_controller_bp)))
    (if (not (Variables|/Game/MotherEarth/GameObjects/ME_HUD.ME_HUD_C|GetISMarquee _asme_hud))
      (Default|SetEnemyOfSelected _asgravity_player_controller_bp self))))

(event EventTick
  (params (DeltaSeconds :type Float%20%28single-precision%29))
  (bind _returnvalue (Game|GetPlayerCameraManager 0))
  (bind _healthbar (Variables|Default|GetHealthBar))
  (bind _spawnthreshold (Variables|Default|GetspawnThreshold))
  (bind _returnvalue_2 (/ _spawnthreshold 4))
  ;[1 1 1] Keep the health bar rotated so the player can see it
  (Utilities|IsValid _healthbar
    (:Is%20Valid
      (Transformation|SetWorldRotation _healthbar (Math|Rotator|FindLookatRotation (Transformation|GetActorLocation (Game|Player|GetPlayerPawn 0)) (Camera|GetCameraLocation _returnvalue)) false false)
      (Transformation|AddRelativeRotation _healthbar (Class|KismetMathLibrary|NegateRotator (Math|Rotator|MakeRotator (.Roll (Math|Rotator|BreakRotator (Camera|GetCameraRotation _returnvalue))) 0.0 0.0)) false false))
    (:Is%20Not%20Valid
      _))
  ;[1 1 1] Logic for spawning enemies
  (if (< (Variables|Default|GetspawnCounter) (Variables|Default|GetrandomizedSpawnThreshold))
    (if (< (Variables|Default|GetenemiesSpawned) (Variables|Default|GetspawnMax))
      (Math|Integer|IncrementInt (Variables|Default|GetspawnCounter)))
    (elif (< (Variables|Default|GetenemiesSpawned) (Variables|Default|GetspawnMax))
      (bind _spawnpoint (CallFunction|GetNextSpawnPoint))
      (bind _returnvalue_3 (Game|SpawnActorfromClass "/Game/MotherEarth/AI/Enemy/GravityEnemyCharacter_BP.GravityEnemyCharacter_BP_C" (Transformation|GetWorldTransform _spawnpoint) "AdjustIfPossibleButDontSpawnIfColliding" 0 0))
      (Utilities|IsValid _returnvalue_3
        (:Is%20Valid
          (Variables|/Game/MotherEarth/AI/Enemy/GravityEnemyCharacter_BP.GravityEnemyCharacter_BP_C|SethomeCrystal _returnvalue_3 self)
          (Variables|Default|SetenemiesSpawned (+ (Variables|Default|GetenemiesSpawned) 1))
          (if (Utilities|IsValid _returnvalue_3)
            (Default|SetGravity _returnvalue_3 "0, 0, 0")
            (Variables|Default|SetspawnCounter 0)
            (Variables|Default|SetrandomizedSpawnThreshold (Math|Random|RandomIntegerinRange (- _spawnthreshold _returnvalue_2) (+ _spawnthreshold _returnvalue_2)))))))))

(fn ConstructionScript)

(fn GetNextSpawnPoint
  (bind _result (Math|Integer|IncrementInt (Variables|Default|GetspawnPointIndex))
    (:%20%20
      (if (> _result 4)
        (Variables|Default|SetspawnPointIndex 0))
      (switch int (Variables|Default|GetspawnPointIndex)
        (:Default
          _)
        (:0
          _)
        (:1
          (return (Variables|Default|GetSpawn%20Point%202)))
        (:2
          (return (Variables|Default|GetSpawn%20Point%203)))
        (:3
          (return (Variables|Default|GetSpawn%20Point%204)))
        (:4
          (return (Variables|Default|GetSpawn%20Point%205))))
      (return (Variables|Default|GetSpawn%20Point%201)))))