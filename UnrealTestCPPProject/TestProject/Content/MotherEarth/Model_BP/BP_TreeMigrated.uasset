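; A tree actor that grows over time and has health, so it can be damaged, healed and destroyed.
; A looping one-second timer counts toward random thresholds, raising the scale per level and swapping to a larger mesh at each new tier.
; Damage reveals and updates an ally health bar widget and destroys the tree at zero, while healing is capped at total health.
; Tick rotates the bar using the player pawn-to-camera direction.
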(event Custom|OnTakeAnyDamage_Event
  (params (DamagedActor :type Actor%20Object%20Reference) (Damage :type Float%20%28single-precision%29) (DamageType :type Damage%20Type%20Object%20Reference) (InstigatedBy :type Controller%20Object%20Reference) (DamageCauser :type Actor%20Object%20Reference))
  ;[1 1 1] Any Actor implementing the BP_HealthBar widget should ideally implement this code
  ;;[1 1 1] If damaged, decrease CurrentHealth and update the health bar, and destroy the actor if health less than 0
  ;;;[1 1 1] Specific for trees
  (Rendering|SetVisibility (Variables|Default|GetHealthBar) true false)
  (bind _output_get (Variables|Default|SetCurrentHealth (- (Variables|Default|GetCurrentHealth) Damage)))
  (bind _asbp_ally_health_bar (Utilities|Casting|CastToBP_AllyHealthBar (UserInterface|GetWidget (Variables|Default|GetHealthBar))))
  (Default|SetHealth _asbp_ally_health_bar (/ _output_get (Variables|Default|GetTotalHealth)))
  (if (<= (Variables|Default|GetCurrentHealth) 0.0)
    (Actor|DestroyActor)))

(event Custom|OnHealDamage
  (params (RestoredHealth :type Float%20%28double-precision%29))
  ;[1 1 1] Any Actor implementing the BP_HealthBar widget should ideally implement this code
  ;;[1 1 1] If healed, increase CurrentHealth and update the health bar, with max possible health being equal to TotalHealth
  (if (<= (+ RestoredHealth (Variables|Default|GetCurrentHealth)) (Variables|Default|GetTotalHealth))
    (Variables|Default|SetCurrentHealth (+ RestoredHealth (Variables|Default|GetCurrentHealth)))
    (else
      (Variables|Default|SetCurrentHealth (Variables|Default|GetTotalHealth))))
  (bind _asbp_ally_health_bar (Utilities|Casting|CastToBP_AllyHealthBar (UserInterface|GetWidget (Variables|Default|GetHealthBar))))
  (Default|SetHealth _asbp_ally_health_bar (/ (Variables|Default|GetCurrentHealth) (Variables|Default|GetTotalHealth))))

(event Custom|treeTick
  ;[1 1 1] Level/Tier up system
  (bind _output_get (Variables|Default|Setcounter (+ (Variables|Default|Getcounter) 1)))
  (if (>= _output_get (Variables|Default|GetlevelUpThreshold))
    (if (< (Variables|Default|GetcurrentLevel) (Variables|Default|GetmaxLevelUps))
      (Transformation|SetActorScale3D (* (Variables|Default|GetstartingScale) (+ (* (Variables|Default|GetcurrentLevel) "0.100000,0.100000,0.100000") "0.800000,0.800000,0.800000")))
      (Variables|Default|Setcounter 0)
      (Variables|Default|SetlevelUpThreshold (+ (Math|Random|RandomInteger 5) 1))
      (Variables|Default|SetcurrentLevel (+ (Variables|Default|GetcurrentLevel) 1))
      (if (== (Variables|Default|GetmaxLevelUps) (Variables|Default|GetcurrentLevel))
        (if (< (Variables|Default|GetcurrentTier) (Variables|Default|GetmaxTier))
          (Variables|Default|SetcurrentLevel 0)
          (Variables|Default|SetcurrentTier (+ (Variables|Default|GetcurrentTier) 1))
          (Transformation|SetActorScale3D (* (Variables|Default|GetstartingScale) (+ (* (Variables|Default|GetcurrentLevel) "0.100000,0.100000,0.100000") "0.800000,0.800000,0.800000")))
          (switch int (Variables|Default|GetcurrentTier)
            (:Default
              (Components|StaticMesh|SetStaticMesh (Variables|Default|GettreeMesh) "/Game/MotherEarth/Meshes/Trees/treeSmall.treeSmall" :!label _label))
            (:0
              (goto _label))
            (:1
              (Components|StaticMesh|SetStaticMesh (Variables|Default|GettreeMesh) "/Game/MotherEarth/Meshes/Trees/treeMid.treeMid"))
            (:2
              (Components|StaticMesh|SetStaticMesh (Variables|Default|GettreeMesh) "/Game/MotherEarth/Meshes/Trees/treeLarge.treeLarge"))))))))

(event EventTick
  (params (DeltaSeconds :type Float%20%28single-precision%29))
  ;[1 1 1] Any Actor implementing the BP_HealthBar widget should ideally implement this code
  ;;[1 1 1] Keep the health bar rotated so the player can see it
  (Transformation|SetWorldRotation (Variables|Default|GetHealthBar) (Math|Rotator|FindLookatRotation (Transformation|GetActorLocation (Game|Player|GetPlayerPawn 0)) (Camera|GetCameraLocation (Game|GetPlayerCameraManager 0))) false false))

(event EventBeginPlay
  (Variables|Default|SetstartingScale (Transformation|GetActorScale3D))
  (Variables|Default|SetHitPoints 0)
  (Variables|Default|Setcounter 0)
  (Variables|Default|SetlevelUpThreshold (+ (Math|Random|RandomInteger 5) 1))
  (Variables|Default|SetcurrentLevel 0)
  (Variables|Default|SetmaxLevelUps 5)
  (Variables|Default|SetmaxTier 2)
  (Variables|Default|SetcurrentTier 0)
  (Transformation|SetActorScale3D (* (Variables|Default|GetstartingScale) (+ (* (Variables|Default|GetcurrentLevel) "0.100000,0.100000,0.100000") "0.800000,0.800000,0.800000")))
  (Utilities|Time|SetTimerbyEvent (delegate Custom|treeTick) 1.0 true)
  (Rendering|SetVisibility (Variables|Default|GetHealthBar) false false)
  ;[1 1 1] Any Actor implementing the BP_HealthBar widget should ideally implement this code
  ;;[1 1 1] If damaged, decrease CurrentHealth and update the health bar, and destroy the actor if health less than 0
  (EventDispatchers|BindEventtoOnTakeAnyDamage (delegate Custom|OnTakeAnyDamage_Event))
  (Variables|Default|SetCurrentHealth (Variables|Default|GetTotalHealth)))

(fn ConstructionScript)