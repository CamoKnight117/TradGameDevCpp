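; BP_MeteorChunk is a short-lived burning meteor fragment actor that burns out after a randomized lifetime.
; BeginPlay randomizes the lifetime around a base value, and Tick counts frames against it, so duration depends on frame rate.
; Past that limit, every Tick deactivates the fire, hides the chunk and re-sets a two-second DestroySelf timer, restarting its countdown.
; Logic to destroy it against land or water tiles is disconnected.
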(event Custom|DestroySelf
  (Actor|DestroyActor))

(event EventTick
  (params (DeltaSeconds :type Float%20%28single-precision%29))
  (bind _count (Variables|Default|Getcount))
  (Math|Integer|IncrementInt _count
    (:%20%20
      (if (> _count (Variables|Default|GetlifetimeRandomized))
        (Components|Activation|Deactivate (Variables|Default|Getfire))
        (Rendering|SetVisibility (Variables|Default|Getchunk) false false)
        (Utilities|Time|SetTimerbyEvent (delegate Custom|DestroySelf) 2.0)))))

(event EventBeginPlay
  (bind _lifetime (Variables|Default|Getlifetime))
  (bind _returnvalue (/ _lifetime 2))
  (Variables|Default|SetlifetimeRandomized (Math|Random|RandomIntegerinRange (- _lifetime _returnvalue) (+ (+ _lifetime _returnvalue) _returnvalue))))

(fn ConstructionScript)