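; Dragon boss that spits fire at nearby player characters and minions; its death shows the YouWin widget and pauses the game.
; Overlaps maintain EnemyList, with a TargetSphere sweep at startup to trigger initial overlaps.
; A looping timer attacks the nearest enemy, playing a montage and re-aiming before spawning BP_DragonFire.
; It heals periodically, shows a camera-facing health bar when damaged, and Ctrl-click sets it as the selection's target.
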(event Custom|OnTakeAnyDamage_Event
  (params (DamagedActor :type Actor%20Object%20Reference) (Damage :type Float%20%28single-precision%29) (DamageType :type Damage%20Type%20Object%20Reference) (InstigatedBy :type Controller%20Object%20Reference) (DamageCauser :type Actor%20Object%20Reference))
  ;[1 1 1] If damaged, decrease CurrentHealth and update the health bar, and destroy the actor if health less than 0
  (Rendering|SetVisibility (Variables|Default|GetHealthBar) true false)
  (bind _output_get (Variables|Default|SetCurrentHealth (- (Variables|Default|GetCurrentHealth) Damage)))
  (bind _asbp_ally_health_bar (Utilities|Casting|CastToBP_AllyHealthBar (UserInterface|GetWidget (Variables|Default|GetHealthBar))))
  (Default|SetHealth _asbp_ally_health_bar (/ _output_get (Variables|Default|GetTotalHealth)))
  (if (<= (Variables|Default|GetCurrentHealth) 0.0)
    (bind _asworld_tile_child (Utilities|Casting|CastToWorldTileChild (Components|GetOwner))
      (:then
        (Default|OnTreeDestroyed _asworld_tile_child))
      (:CastFailed
        _))
    (Viewport|RemoveAllWidgets)
    (bind _returnvalue (UserInterface|CreateWidget "/Game/MotherEarth/UI/YouWin.YouWin_C" (Game|GetPlayerController 0)))
    (UserInterface|Viewport|AddtoViewport _returnvalue 0)
    (Game|SetGamePaused true)
    (Actor|DestroyActor)))

(event Custom|sweepBack
  ;[1 1 1] Move the collision sphere away, then back to trigger begin overlap events
  (Transformation|SetRelativeLocation (Variables|Default|GettargetSphere) "0, 0, 0" true false))

(event Custom|OnHealDamage
  (params (RestoredHealth :type Float%20%28double-precision%29))
  (bind _healthbar (Variables|Default|GetHealthBar))
  ;[1 1 1] If healed, increase CurrentHealth and update the health bar, with max possible health being equal to TotalHealth
  (if (<= (+ RestoredHealth (Variables|Default|GetCurrentHealth)) (Variables|Default|GetTotalHealth))
    (Variables|Default|SetCurrentHealth (+ RestoredHealth (Variables|Default|GetCurrentHealth)))
    (else
      (Variables|Default|SetCurrentHealth (Variables|Default|GetTotalHealth))
      (Rendering|SetVisibility _healthbar false false)))
  (bind _asbp_ally_health_bar (Utilities|Casting|CastToBP_AllyHealthBar (UserInterface|GetWidget _healthbar)))
  (Default|SetHealth _asbp_ally_health_bar (/ (Variables|Default|GetCurrentHealth) (Variables|Default|GetTotalHealth))))

(event Custom|Attack
  (if (> (Utilities|Array|Length (Variables|Default|GetenemyList)) 0)
    (CallFunction|FireProjectile (Transformation|GetActorLocation (.ReturnValue (Actor|FindNearestActor (Transformation|GetWorldLocation (Variables|Default|GetDefaultSceneRoot)) (Variables|Default|GetenemyList)))))))

(event EventActorOnReleased
  (params (ButtonReleased :type Key%20Structure :default "None"))
  ;[1 1 1] Targeting logic
  (bind _asgravity_player_controller_bp (Utilities|Casting|CastToGravityPlayerController_BP (Game|GetPlayerController 0)))
  (if (Variables|/Game/MotherEarth/GameObjects/GravityPlayerController_BP.GravityPlayerController_BP_C|GetleftCtrlPressed _asgravity_player_controller_bp)
    (bind _asme_hud (Utilities|Casting|CastToME_HUD (HUD|GetHUD _asgravity_player_controller_bp)))
    (if (not (Variables|/Game/MotherEarth/GameObjects/ME_HUD.ME_HUD_C|GetISMarquee _asme_hud))
      (Default|SetEnemyOfSelected _asgravity_player_controller_bp self))))

(event EventTick
  (params (DeltaSeconds :type Float%20%28single-precision%29))
  (bind _returnvalue (Game|GetPlayerCameraManager 0))
  (bind _healthbar (Variables|Default|GetHealthBar))
  (bind _defaultsceneroot (Variables|Default|GetDefaultSceneRoot))
  (bind _relativerotation (Variables|/Script/Engine.SceneComponent|GetRelativeRotation _defaultsceneroot))
  ;[1 1 1] Keep the health bar rotated so the player can see it
  (Transformation|SetWorldRotation _healthbar (Math|Rotator|FindLookatRotation (Transformation|GetActorLocation (Game|Player|GetPlayerPawn 0)) (Camera|GetCameraLocation _returnvalue)) false false)
  (Transformation|AddRelativeRotation _healthbar (Class|KismetMathLibrary|NegateRotator (Math|Rotator|MakeRotator (.Roll (Math|Rotator|BreakRotator (Camera|GetCameraRotation _returnvalue))) 0.0 0.0)) false false)
  (if (> (Utilities|Array|Length (Variables|Default|GetenemyList)) 0)
    (Transformation|SetRelativeRotation _defaultsceneroot (Math|Rotator|MakeRotator (.roll _relativerotation) (.pitch _relativerotation) (.yaw _relativerotation)) false false)))

(event EventBeginPlay
  (Utilities|Time|SetTimerbyEvent (delegate Custom|Attack) 6e+01 true)
  (Rendering|SetVisibility (Variables|Default|GetSelectionCircle) false false)
  (Variables|Default|SetactorStartingTransform (Transformation|GetActorTransform))
  (Utilities|Time|SetTimerbyFunctionName 0 "healOverTime" 3.0)
  (Rendering|SetVisibility (Variables|Default|GetHealthBar) false false)
  ;[1 1 1] If damaged, decrease CurrentHealth and update the health bar, and destroy the actor if health less than 0
  (EventDispatchers|BindEventtoOnTakeAnyDamage (delegate Custom|OnTakeAnyDamage_Event))
  (Variables|Default|SetCurrentHealth (Variables|Default|GetTotalHealth))
  ;[1 1 1] Move the collision sphere away, then back to trigger begin overlap events
  (Transformation|SetRelativeLocation (Variables|Default|GettargetSphere) (* (Transformation|GetActorLocation) 5.0) false true)
  (Utilities|Time|SetTimerbyEvent (delegate Custom|sweepBack) 1.0))

(event Collision|EventActorBeginOverlap
  (params (OtherActor :type Actor%20Object%20Reference))
  (Utilities|Casting|CastToGravityPlayerCharacter_BP OtherActor
    (:then
      _)
    (:CastFailed
      (Utilities|Casting|CastToGravityMinionCharacter_BP OtherActor)))
  (Utilities|Array|Add (Variables|Default|GetenemyList) OtherActor))

(event Collision|EventActorEndOverlap
  (params (OtherActor :type Actor%20Object%20Reference))
  (Utilities|Casting|CastToGravityPlayerCharacter_BP OtherActor
    (:then
      _)
    (:CastFailed
      (Utilities|Casting|CastToGravityMinionCharacter_BP OtherActor)))
  (Utilities|Array|RemoveItem (Variables|Default|GetenemyList) OtherActor))

(fn ConstructionScript)

(fn HealOverTime
  (Utilities|IsValid self
    (:Is%20Valid
      (Utilities|Time|SetTimerbyFunctionName 0 "healOverTime" 3.0)
      (CallFunction|OnHealDamage (Variables|Default|GetHealRate)))))

(fn FireProjectile
  (params (targetLocation :type Vector))
  (Variables|Default|SetProjectile%20Rotation (Math|Rotator|FindLookatRotation (Transformation|GetWorldLocation (Variables|Default|GetspitSpawn)) targetLocation))
  (Utilities|Time|SetTimerbyFunctionName 0 "createProjectile" 1.0)
  (Components|Animation|PlayAnimation (Variables|Default|GetSkeletalMesh) "/Game/MotherEarth/Model_BP/CharModelsAndAnims/Ani/Dragon/AttackDra_Montage.AttackDra_Montage" false)
  (Utilities|Time|SetTimerbyFunctionName 0 "resumeIdleAnim" 2.0))

(fn CreateProjectile
  (CallFunction|UpdateTargetLocation)
  (Game|SpawnActorfromClass "/Game/MotherEarth/Model_BP/BP_DragonFire.BP_DragonFire_C" (Math|Transform|MakeTransform (Transformation|GetWorldLocation (Variables|Default|GetspitSpawn)) (Variables|Default|GetProjectile%20Rotation) "1.000000,1.000000,1.000000") "Undefined" 0 0))

(fn ResumeIdleAnim
  (Components|Animation|PlayAnimation (Variables|Default|GetSkeletalMesh) "/Game/MotherEarth/Model_BP/CharModelsAndAnims/Ani/Dragon/Idle.Idle" true))

(fn UpdateTargetLocation
  (bind _enemylist (Variables|Default|GetenemyList))
  (if (> (Utilities|Array|Length _enemylist) 0)
    (Variables|Default|SetProjectile%20Rotation (Math|Rotator|FindLookatRotation (Transformation|GetWorldLocation (Variables|Default|GetspitSpawn)) (Transformation|GetActorLocation (.ReturnValue (Actor|FindNearestActor (Transformation|GetWorldLocation (Variables|Default|GetDefaultSceneRoot)) _enemylist)))))))