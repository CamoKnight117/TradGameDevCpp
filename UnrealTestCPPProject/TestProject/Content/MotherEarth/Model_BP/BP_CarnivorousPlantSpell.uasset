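; BP_CarnivorousPlantSpell is a short-lived spell actor that plants a carnivorous plant on grass world tiles.
; Overlapping a grass WorldTileChild asks the tile to spawn the plant at the spell's location, then destroys the spell.
; Overlapping a non-grass tile sets the player's CarnivorousSpellCounter to its max without destroying the spell.
; A randomized, frame-counted DeathTimer destroys the actor when it runs out.
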(event Collision|EventActorBeginOverlap
  (params (OtherActor :type Actor%20Object%20Reference))
  (bind _asworld_tile_child (Utilities|Casting|CastToWorldTileChild OtherActor))
  (if (Variables|/Game/MotherEarth/WorldTileChild.WorldTileChild_C|GetIsGrass _asworld_tile_child)
    (Default|SpawnCarnivorePlant _asworld_tile_child (Transformation|GetActorLocation))
    (Actor|DestroyActor)
    (else
      (bind _asgravity_player_character_bp (Utilities|Casting|CastToGravityPlayerCharacter_BP (Game|Player|GetPlayerPawn 0)))
      (Variables|/Game/MotherEarth/GravityPlayerCharacter_BP.GravityPlayerCharacter_BP_C|SetcarnivorousSpellCounter _asgravity_player_character_bp (Variables|/Game/MotherEarth/GravityPlayerCharacter_BP.GravityPlayerCharacter_BP_C|GetcarnivorousSpellMax _asgravity_player_character_bp)))))

(event EventTick
  (params (DeltaSeconds :type Float%20%28single-precision%29))
  (Variables|Default|SetdeathTimer (- (Variables|Default|GetdeathTimer) 1))
  (if (< (Variables|Default|GetdeathTimer) 0)
    (Actor|DestroyActor)))

(event EventBeginPlay
  (Variables|Default|SetdeathTimer (Math|Random|RandomIntegerinRange 20 35)))

(fn ConstructionScript)