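; Region actor that groups overlapping world tiles and flips the region between green, neutral and enemy states by tile percentages.
; Overlaps register tiles, enemies, base, pillar markers and crystal, and pass them the movable mountain and bridge; BeginPlay sweeps the collider to trigger these.
; After a delay, tiles receive their region.
; CheckTileConditions applies grass, red and planted thresholds to toggle base and pillars, first forcing enemy state if the base starts as enemy.
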(event Custom|Configure%20Region%20Tiles
  (bind _result (Utilities|Set|ToArray (Variables|Default|GetcollidingTiles)))
  (for _array_element _result
    (bind _asworld_tile_child (Utilities|Casting|CastToWorldTileChild _array_element))
    (Default|SetRegion _asworld_tile_child self))
  (CallFunction|CheckTileConditions))

(event Custom|sweepBack
  ;[1 1 1] Move the collision sphere away, then back to trigger begin overlap events
  (Transformation|SetRelativeLocation (Variables|Default|GetregionSizeCollider) "0, 0, 0" true false))

(event EventBeginPlay
  (Utilities|Time|SetTimerbyEvent (delegate Custom|Configure%20Region%20Tiles) 2.0)
  (Variables|Default|SetregionActive false)
  (Variables|Default|SetregionEnemyActive false)
  ;[1 1 1] Move the collision sphere away, then back to trigger begin overlap events
  (Transformation|SetRelativeLocation (Variables|Default|GetregionSizeCollider) (* (Transformation|GetActorLocation) 5.0) false true)
  (Utilities|Time|SetTimerbyEvent (delegate Custom|sweepBack) 1.0)
  (Utilities|FlowControl|Delay 0.1)
  (Utilities|Set|AddItems (Variables|Default|GetEnemyList) (Collision|GetOverlappingActors (Variables|Default|GetregionSizeCollider) "/Game/MotherEarth/AI/Enemy/GravityEnemyCharacter_BP.GravityEnemyCharacter_BP_C" :!class /Script/Engine.PrimitiveComponent)))

(event Collision|EventActorBeginOverlap
  (params (OtherActor :type Actor%20Object%20Reference))
  ;[1 1 1] The begin overlap and end overlap events are used to keep track of which tiles belong to a given region
  (bind _asworld_tile_child (Utilities|Casting|CastToWorldTileChild OtherActor)
    (:then
      (Utilities|Set|Add (Variables|Default|GetcollidingTiles) _asworld_tile_child))
    (:CastFailed
      (bind _asgravity_enemy_character_bp (Utilities|Casting|CastToGravityEnemyCharacter_BP OtherActor)
        (:then
          (Utilities|Set|Add (Variables|Default|GetEnemyList) _asgravity_enemy_character_bp))
        (:CastFailed
          (bind _asbp_stone_henge_base (Utilities|Casting|CastToBP_StoneHengeBase OtherActor)
            (:then
              (Variables|Default|SetmyBase _asbp_stone_henge_base))
            (:CastFailed
              (bind _asbp_pillar_marker_grass (Utilities|Casting|CastToBP_PillarMarkerGrass OtherActor)
                (:then
                  (bind _output_get (Variables|Default|SetmyPillarMarkerGrass _asbp_pillar_marker_grass))
                  (Utilities|IsValid (Variables|Default|GetmovableMountain)
                    (:Is%20Valid
                      (Variables|/Game/MotherEarth/Model_BP/BP_PillarMarkerGrass.BP_PillarMarkerGrass_C|SetmovableMountain _output_get (Variables|Default|GetmovableMountain)))
                    (:Is%20Not%20Valid
                      _))
                  (Utilities|IsValid (Variables|Default|GetmovableBridge)
                    (:Is%20Valid
                      (Variables|/Game/MotherEarth/Model_BP/BP_PillarMarkerGrass.BP_PillarMarkerGrass_C|SetmovableBridge _output_get (Variables|Default|GetmovableBridge)))))
                (:CastFailed
                  (bind _asbp_pillar_marker_plants (Utilities|Casting|CastToBP_PillarMarkerPlants OtherActor)
                    (:then
                      (bind _output_get_2 (Variables|Default|SetmyPillarMarkerPlants _asbp_pillar_marker_plants))
                      (Utilities|IsValid (Variables|Default|GetmovableMountain)
                        (:Is%20Valid
                          (Variables|/Game/MotherEarth/Model_BP/BP_PillarMarkerPlants.BP_PillarMarkerPlants_C|SetmovableMountain _output_get_2 (Variables|Default|GetmovableMountain)))
                        (:Is%20Not%20Valid
                          _))
                      (Utilities|IsValid (Variables|Default|GetmovableBridge)
                        (:Is%20Valid
                          (Variables|/Game/MotherEarth/Model_BP/BP_PillarMarkerPlants.BP_PillarMarkerPlants_C|SetmovableBridge _output_get_2 (Variables|Default|GetmovableBridge)))))
                    (:CastFailed
                      (bind _asbp_moving_mountain (Utilities|Casting|CastToBP_MovingMountain OtherActor)
                        (:then
                          (if (Variables|Default|GetsetManually)
                            _
                            (else
                              (bind _output_get_3 (Variables|Default|SetmovableMountain _asbp_moving_mountain))))
                          (Utilities|IsValid _output_get_2
                            (:Is%20Valid
                              (Variables|/Game/MotherEarth/Model_BP/BP_PillarMarkerPlants.BP_PillarMarkerPlants_C|SetmovableMountain _output_get_2 _output_get_3))
                            (:Is%20Not%20Valid
                              _))
                          (Utilities|IsValid _output_get
                            (:Is%20Valid
                              (Variables|/Game/MotherEarth/Model_BP/BP_PillarMarkerGrass.BP_PillarMarkerGrass_C|SetmovableMountain _output_get _output_get_3))
                            (:Is%20Not%20Valid
                              _))
                          (Utilities|IsValid (Variables|Default|GetenemyCrystal)
                            (:Is%20Valid
                              (Variables|/Game/MotherEarth/Model_BP/BP_Crystal.BP_Crystal_C|SetmovableMountain (Variables|Default|GetenemyCrystal) (Variables|Default|GetmovableMountain)))))
                        (:CastFailed
                          (bind _asbp_activated_bridge (Utilities|Casting|CastToBP_ActivatedBridge OtherActor)
                            (:then
                              (Default|MovetoStartingPosition _asbp_activated_bridge)
                              (if (Variables|Default|GetsetManually)
                                _
                                (else
                                  (bind _output_get_4 (Variables|Default|SetmovableBridge _asbp_activated_bridge))))
                              (Utilities|IsValid _output_get_2
                                (:Is%20Valid
                                  (Variables|/Game/MotherEarth/Model_BP/BP_PillarMarkerPlants.BP_PillarMarkerPlants_C|SetmovableBridge _output_get_2 _output_get_4))
                                (:Is%20Not%20Valid
                                  _))
                              (Utilities|IsValid _output_get
                                (:Is%20Valid
                                  (Variables|/Game/MotherEarth/Model_BP/BP_PillarMarkerGrass.BP_PillarMarkerGrass_C|SetmovableBridge _output_get _output_get_4))
                                (:Is%20Not%20Valid
                                  _))
                              (Utilities|IsValid (Variables|Default|GetenemyCrystal)
                                (:Is%20Valid
                                  (Variables|/Game/MotherEarth/Model_BP/BP_Crystal.BP_Crystal_C|SetmovableBridge (Variables|Default|GetenemyCrystal) (Variables|Default|GetmovableBridge)))))
                            (:CastFailed
                              (bind _asbp_crystal (Utilities|Casting|CastToBP_Crystal OtherActor))
                              (bind _output_get_5 (Variables|Default|SetenemyCrystal _asbp_crystal))
                              (Utilities|IsValid (Variables|Default|GetmovableMountain)
                                (:Is%20Valid
                                  (Variables|/Game/MotherEarth/Model_BP/BP_Crystal.BP_Crystal_C|SetmovableMountain _output_get_5 (Variables|Default|GetmovableMountain)))
                                (:Is%20Not%20Valid
                                  _))
                              (Utilities|IsValid (Variables|Default|GetmovableBridge)
                                (:Is%20Valid
                                  (Variables|/Game/MotherEarth/Model_BP/BP_Crystal.BP_Crystal_C|SetmovableBridge _output_get_5 (Variables|Default|GetmovableBridge)))))))))))))))))))

(event Collision|EventActorEndOverlap
  (params (OtherActor :type Actor%20Object%20Reference))
  ;[1 1 1] The begin overlap and end overlap events are used to keep track of which tiles belong to a given region
  (bind _asworld_tile_child (Utilities|Casting|CastToWorldTileChild OtherActor)
    (:then
      (Utilities|Set|Remove (Variables|Default|GetcollidingTiles) _asworld_tile_child))
    (:CastFailed
      (bind _asgravity_enemy_character_bp (Utilities|Casting|CastToGravityEnemyCharacter_BP OtherActor))
      (Utilities|Set|Remove (Variables|Default|GetEnemyList) _asgravity_enemy_character_bp))))

(fn ConstructionScript)

(fn CheckTileConditions
  (bind _mypillarmarkergrass (Variables|Default|GetmyPillarMarkerGrass))
  (bind _mypillarmarkergrass_2 (Variables|Default|GetmyPillarMarkerGrass))
  (bind _mybase (Variables|Default|GetmyBase))
  (bind _mybase_2 (Variables|Default|GetmyBase))
  (bind _mybase_3 (Variables|Default|GetmyBase))
  (bind _mybase_4 (Variables|Default|GetmyBase))
  (bind _mypillarmarkergrass_3 (Variables|Default|GetmyPillarMarkerGrass))
  (bind _mypillarmarkerplants (Variables|Default|GetmyPillarMarkerPlants))
  (bind _mypillarmarkerplants_2 (Variables|Default|GetmyPillarMarkerPlants))
  (bind _mypillarmarkerplants_3 (Variables|Default|GetmyPillarMarkerPlants))
  ;[1 1 1] Logic for checking if a region should "flip" to be good or bad
  (if (> (Utilities|Set|Length (Variables|Default|GetcollidingTiles)) 0)
    (Variables|Default|SettotalGreenTiles 0)
    (Variables|Default|SettotalRedTiles 0)
    (Variables|Default|SettotalPlantedTiles 0)
    (bind _result (Utilities|Set|ToArray (Variables|Default|GetcollidingTiles)))
    (for _array_element _result
      (bind _asworld_tile_child (Utilities|Casting|CastToWorldTileChild _array_element))
      (if (Variables|/Game/MotherEarth/WorldTileChild.WorldTileChild_C|GetIsGrass _asworld_tile_child)
        (Variables|Default|SettotalGreenTiles (+ 1 (Variables|Default|GettotalGreenTiles)))
        (if (Variables|/Game/MotherEarth/WorldTileChild.WorldTileChild_C|GethasPlants _asworld_tile_child)
          (Math|Integer|IncrementInt (Variables|Default|GettotalPlantedTiles)))
        (elif (Variables|/Game/MotherEarth/WorldTileChild.WorldTileChild_C|GetisRed _asworld_tile_child)
          (Variables|Default|SettotalRedTiles (+ 1 (Variables|Default|GettotalRedTiles))))))
    (Utilities|IsValid _mybase_3
      (:Is%20Valid
        (if (Variables|/Game/MotherEarth/Model_BP/BP_StoneHengeBase.BP_StoneHengeBase_C|GetstartAsEnemy _mybase_3)
          (if (Variables|Default|GethasBeenFlipped)
            (if (>= (* (/ (Math|Conversions|ToFloat(Integer) (Variables|Default|GettotalGreenTiles)) (Math|Conversions|ToFloat(Integer) (Utilities|Set|Length (Variables|Default|GetcollidingTiles)))) 1e+02) (Variables|Default|GetchangeToGreenThreshold)) :!label _label
              (if (Variables|Default|GetregionActive)
                (if (>= (* (/ (Math|Conversions|ToFloat(Integer) (Variables|Default|GettotalPlantedTiles)) (Math|Conversions|ToFloat(Integer) (Utilities|Set|Length (Variables|Default|GetcollidingTiles)))) 1e+02) (Variables|Default|GetplantedTilesThreshold)) :!label _label_2
                  (Utilities|IsValid _mypillarmarkerplants
                    (:Is%20Valid
                      (Default|Activate _mypillarmarkerplants))))
                (else
                  (Variables|Default|SetregionEnemyActive false)
                  (Variables|Default|SetregionActive true)
                  (if (Utilities|IsValid _mybase_2)
                    (Default|ActivateBase _mybase_2)
                    (Variables|Default|SethasBeenFlipped true))
                  (Utilities|IsValid _mypillarmarkergrass_3
                    (:Is%20Valid
                      (Default|Activate _mypillarmarkergrass_3)
                      (Variables|Default|SethasBeenFlipped true))
                    (:Is%20Not%20Valid
                      _))
                  (Utilities|IsValid _mypillarmarkerplants
                    (:Is%20Valid
                      (goto _label_2))
                    (:Is%20Not%20Valid
                      _))))
              (Variables|Default|SethasBeenFlipped true)
              (elif (<= (* (/ (Math|Conversions|ToFloat(Integer) (Variables|Default|GettotalGreenTiles)) (Math|Conversions|ToFloat(Integer) (Utilities|Set|Length (Variables|Default|GetcollidingTiles)))) 1e+02) (Variables|Default|GetmaintainGreenThreshold))
                (if (Variables|Default|GetregionActive)
                  (Variables|Default|SetregionEnemyActive false)
                  (Variables|Default|SetregionActive false)
                  (if (Utilities|IsValid _mybase_4)
                    (Default|DeactivateBase _mybase_4)
                    (Variables|Default|SethasBeenFlipped true))
                  (Utilities|IsValid _mypillarmarkergrass_2
                    (:Is%20Valid
                      (Default|Deactivate _mypillarmarkergrass_2)
                      (Variables|Default|SethasBeenFlipped true))
                    (:Is%20Not%20Valid
                      _))
                  (Utilities|IsValid _mypillarmarkerplants_3
                    (:Is%20Valid
                      (Default|Deactivate _mypillarmarkerplants_3))
                    (:Is%20Not%20Valid
                      _))
                  (Variables|Default|SethasBeenFlipped true)
                  (elif (>= (* (/ (Math|Conversions|ToFloat(Integer) (Variables|Default|GettotalRedTiles)) (Math|Conversions|ToFloat(Integer) (Utilities|Set|Length (Variables|Default|GetcollidingTiles)))) 1e+02) (Variables|Default|GetchangeToEnemyThreshold))
                    (if (not (Variables|Default|GetregionEnemyActive))
                      (Variables|Default|SetregionEnemyActive true :!label _label_3)
                      (Variables|Default|SetregionActive false)
                      (if (Utilities|IsValid _mybase)
                        (Default|ActivateEnemyBase _mybase)
                        (Variables|Default|SethasBeenFlipped true))
                      (Utilities|IsValid _mypillarmarkergrass
                        (:Is%20Valid
                          (Default|EnemyActivate _mypillarmarkergrass)
                          (Variables|Default|SethasBeenFlipped true))
                        (:Is%20Not%20Valid
                          _))
                      (Utilities|IsValid _mypillarmarkerplants_2
                        (:Is%20Valid
                          (Default|EnemyActivate _mypillarmarkerplants_2))
                        (:Is%20Not%20Valid
                          _))
                      (Variables|Default|SethasBeenFlipped true))))))
            (else
              (goto _label_3)))
          (else
            (goto _label))))
      (:Is%20Not%20Valid
        (goto _label)))))