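; Meteor shower zone that drops meteors toward the world origin while the player character overlaps it.
; Tick counts frames up to a threshold, re-randomized within a quarter of its base value, then spawns a meteor.
; Each meteor starts at SpawnRadius along the origin-to-point direction of one of six random spawn components, receiving that component and the system as owner.
; SpawnMeteorEnemy spawns a gravity gorilla enemy at a given point but is not called here.
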(event EventBeginPlay
  (bind _meteorshowerthreshold (Variables|Default|GetmeteorShowerThreshold))
  (bind _returnvalue (/ _meteorshowerthreshold 4))
  (Variables|Default|SetmeteorThresholdRandomized (Math|Random|RandomIntegerinRange (- _meteorshowerthreshold _returnvalue) (+ _meteorshowerthreshold _returnvalue))))

(event Collision|EventActorBeginOverlap
  (params (OtherActor :type Actor%20Object%20Reference))
  (Utilities|Casting|CastToGravityPlayerCharacter_BP OtherActor)
  (Variables|Default|Setactive true))

(event EventTick
  (params (DeltaSeconds :type Float%20%28single-precision%29))
  (bind _meteorshowerthreshold (Variables|Default|GetmeteorShowerThreshold))
  (bind _returnvalue (/ _meteorshowerthreshold 4))
  (if (Variables|Default|Getactive)
    (bind _result (Math|Integer|IncrementInt (Variables|Default|GetmeteorCount))
      (:%20%20
        (if (> _result (Variables|Default|GetmeteorThresholdRandomized))
          (Variables|Default|SetmeteorThresholdRandomized (Math|Random|RandomIntegerinRange (- _meteorshowerthreshold _returnvalue) (+ _meteorshowerthreshold _returnvalue)))
          (CallFunction|SpawnMeteor))))))

(event Collision|EventActorEndOverlap
  (params (OtherActor :type Actor%20Object%20Reference))
  (Utilities|Casting|CastToGravityPlayerCharacter_BP OtherActor)
  (Variables|Default|Setactive false))

(fn ConstructionScript)

(fn SpawnMeteor
  (bind _spawnlocation (CallFunction|GetRandomSpawnComponent))
  (bind _returnvalue (Game|SpawnActorfromClass "/Game/MotherEarth/Model_BP/BP_Meteor.BP_Meteor_C" (Math|Transform|MakeTransform (* (Math|Vector|Normalize (Transformation|GetWorldLocation _spawnlocation)) (Variables|Default|GetspawnRadius)) (Math|Rotator|FindLookatRotation (* (Math|Vector|Normalize (Transformation|GetWorldLocation _spawnlocation)) (Variables|Default|GetspawnRadius)) (Math|Vector|VectorZero)) "1.000000,1.000000,1.000000") "Undefined" 0 0))
  (Variables|/Game/MotherEarth/Model_BP/BP_Meteor.BP_Meteor_C|SetmeteorOwner _returnvalue self)
  (Variables|/Game/MotherEarth/Model_BP/BP_Meteor.BP_Meteor_C|SetenemySpawnPoint _returnvalue _spawnlocation)
  (Variables|Default|SetmeteorCount 0))

(fn GetRandomSpawnComponent
  (switch int (Math|Random|RandomIntegerinRange 0 5)
    (:Default
      _)
    (:0
      _)
    (:1
      (return (Variables|Default|Getspawn1)))
    (:2
      (return (Variables|Default|Getspawn3)))
    (:3
      (return (Variables|Default|Getspawn6)))
    (:4
      (return (Variables|Default|Getspawn5)))
    (:5
      (return (Variables|Default|Getspawn4))))
  (return (Variables|Default|Getspawn2)))

(fn SpawnMeteorEnemy
  (params (spawnLocation :type Capsule%20Component%20Object%20Reference))
  (bind _returnvalue (Game|SpawnActorfromClass "/Game/MotherEarth/AI/Enemy/GravityEnemyGorilla_BP.GravityEnemyGorilla_BP_C" (Transformation|GetWorldTransform spawnLocation) "AdjustIfPossibleButAlwaysSpawn" 0 0))
  (Default|SetGravity _returnvalue "0, 0, 0"))