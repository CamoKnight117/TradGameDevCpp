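; Stonehenge base that spawns minions while player-active or enemies while enemy-active, showing a green field or fires respectively.
; Tick counts frames toward a threshold randomized by ±25%, then spawns a capped, zero-gravity unit homed to this base at one of five cycled points.
; A radial widget shows spawn progress and, with its background, rotates toward the camera.
; Releasing a click with left Ctrl held selects the base, unless marquee selection is active.
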(event EventBeginPlay
  (Utilities|Array|Add (Variables|Default|GetspawnPointArray) (Variables|Default|GetspawnPoint1)))

(event EventTick
  (params (DeltaSeconds :type Float%20%28single-precision%29))
  (bind _returnvalue (Game|GetPlayerCameraManager 0))
  (bind _returnvalue_2 (Game|Player|GetPlayerPawn 0))
  (bind _spawnthreshold (Variables|Default|GetspawnThreshold))
  (bind _radialspawnwidget (Variables|Default|GetRadialSpawnWidget))
  (bind _backgroundwidget (Variables|Default|GetBackgroundWidget))
  (bind _returnvalue_3 (Transformation|GetActorLocation _returnvalue_2))
  (bind _returnvalue_4 (Camera|GetCameraLocation _returnvalue))
  (bind _returnvalue_5 (Camera|GetCameraRotation _returnvalue))
  (bind _returnvalue_6 (/ _spawnthreshold 4))
  (bind _returnvalue_7 (Math|Rotator|FindLookatRotation _returnvalue_3 _returnvalue_4))
  (bind _roll (Math|Rotator|BreakRotator _returnvalue_5))
  (bind _returnvalue_8 (Math|Rotator|MakeRotator _roll 0.0 0.0))
  (bind _returnvalue_9 (Class|KismetMathLibrary|NegateRotator _returnvalue_8))
  ;[1 1 1] Keep the radial rotated so the player can see it
  (Transformation|SetWorldRotation _radialspawnwidget _returnvalue_7 false false)
  (Transformation|AddRelativeRotation _radialspawnwidget _returnvalue_9 false false)
  (Transformation|SetWorldRotation _backgroundwidget _returnvalue_7 false false)
  (Transformation|AddRelativeRotation _backgroundwidget _returnvalue_9 false false)
  (if (or (Variables|Default|GetplayerActive) (Variables|Default|GetenemyActive))
    (if (< (Variables|Default|GetspawnCounter) (Variables|Default|GetrandomizedSpawnThreshold))
      (if (and (< (Variables|Default|GetminionsSpawned) (Variables|Default|GetspawnMax)) (< (Variables|Default|GetenemiesSpawned) (Variables|Default|GetspawnMax)))
        (Math|Integer|IncrementInt (Variables|Default|GetspawnCounter)
          (:%20%20
            (bind _aswb_radial_bar (Utilities|Casting|CastToWB_RadialBar (UserInterface|GetWidget (Variables|Default|GetRadialSpawnWidget))))
            (Default|SetPercent _aswb_radial_bar (/ (Math|Conversions|ToFloat(Integer) (Variables|Default|GetspawnCounter)) (Math|Conversions|ToFloat(Integer) (Variables|Default|GetrandomizedSpawnThreshold))) false))))
      (elif (Variables|Default|GetplayerActive)
        (if (< (Variables|Default|GetminionsSpawned) (Variables|Default|GetspawnMax))
          (bind _spawnpoint (CallFunction|GetNextSpawnPoint))
          (bind _returnvalue_10 (Game|SpawnActorfromClass "/Game/MotherEarth/AI/Minion/GravityMinionCharacter_BP.GravityMinionCharacter_BP_C" (Transformation|GetWorldTransform _spawnpoint) "AdjustIfPossibleButDontSpawnIfColliding" 0 0))
          (Utilities|IsValid _returnvalue_10
            (:Is%20Valid
              (Variables|/Game/MotherEarth/AI/Minion/GravityMinionCharacter_BP.GravityMinionCharacter_BP_C|SethomeBase _returnvalue_10 self)
              (Variables|Default|SetminionsSpawned (+ (Variables|Default|GetminionsSpawned) 1))
              (if (Utilities|IsValid _returnvalue_10)
                (Default|SetGravity _returnvalue_10 "0, 0, 0")
                (Variables|Default|SetspawnCounter 0 :!label _label)
                (Variables|Default|SetrandomizedSpawnThreshold (Math|Random|RandomIntegerinRange (- _spawnthreshold _returnvalue_6) (+ _spawnthreshold _returnvalue_6)))
                (bind _aswb_radial_bar_2 (Utilities|Casting|CastToWB_RadialBar (UserInterface|GetWidget (Variables|Default|GetRadialSpawnWidget))))
                (Default|SetPercent _aswb_radial_bar_2 (/ (Math|Conversions|ToFloat(Integer) (Variables|Default|GetspawnCounter)) (Math|Conversions|ToFloat(Integer) (Variables|Default|GetrandomizedSpawnThreshold))) false)))))
        (elif (Variables|Default|GetenemyActive)
          (if (< (Variables|Default|GetenemiesSpawned) (Variables|Default|GetspawnMax))
            (bind _spawnpoint_2 (CallFunction|GetNextSpawnPoint))
            (bind _returnvalue_11 (Game|SpawnActorfromClass "/Game/MotherEarth/AI/Enemy/GravityEnemyCharacter_BP.GravityEnemyCharacter_BP_C" (Transformation|GetWorldTransform _spawnpoint_2) "AdjustIfPossibleButDontSpawnIfColliding" 0 0))
            (Utilities|IsValid _returnvalue_11
              (:Is%20Valid
                (Variables|/Game/MotherEarth/AI/Enemy/GravityEnemyCharacter_BP.GravityEnemyCharacter_BP_C|SethomeBase _returnvalue_11 self)
                (Variables|Default|SetenemiesSpawned (+ (Variables|Default|GetenemiesSpawned) 1))
                (if (Utilities|IsValid _returnvalue_11)
                  (Default|SetGravity _returnvalue_11 "0, 0, 0")
                  (goto _label))))))))))

(event EventActorOnReleased
  (params (ButtonReleased :type Key%20Structure :default "None"))
  (bind _asgravity_player_controller_bp (Utilities|Casting|CastToGravityPlayerController_BP (Game|GetPlayerController 0)))
  (if (Variables|/Game/MotherEarth/GameObjects/GravityPlayerController_BP.GravityPlayerController_BP_C|GetleftCtrlPressed _asgravity_player_controller_bp)
    (bind _asme_hud (Utilities|Casting|CastToME_HUD (HUD|GetHUD _asgravity_player_controller_bp)))
    (if (not (Variables|/Game/MotherEarth/GameObjects/ME_HUD.ME_HUD_C|GetISMarquee _asme_hud))
      (Default|SetBaseOfSelected _asgravity_player_controller_bp self))))

(fn ConstructionScript)

(fn ActivateBase
  (bind _spawnthreshold (Variables|Default|GetspawnThreshold))
  (bind _returnvalue (/ _spawnthreshold 4))
  (Variables|Default|SetspawnCounter 0)
  (Variables|Default|SetplayerActive true)
  (Variables|Default|SetenemyActive false)
  (CallFunction|StopFire)
  (Components|Activation|Activate (Variables|Default|GetgreenField) false)
  (Variables|Default|SetrandomizedSpawnThreshold (Math|Random|RandomIntegerinRange (- _spawnthreshold _returnvalue) (+ _spawnthreshold _returnvalue))))

(fn DeactivateBase
  (Variables|Default|SetspawnCounter 0)
  (Variables|Default|SetplayerActive false)
  (Variables|Default|SetenemyActive false)
  (Components|Activation|Deactivate (Variables|Default|GetgreenField)))

(fn ActivateEnemyBase
  (Variables|Default|SetspawnCounter 0)
  (Variables|Default|SetplayerActive false)
  (Variables|Default|SetenemyActive true)
  (CallFunction|StartFire)
  (Components|Activation|Deactivate (Variables|Default|GetgreenField)))

(fn StartFire
  (Variables|Default|SetonFire true)
  (Components|Activation|Activate (Variables|Default|Getfire2) false)
  (Components|Activation|Activate (Variables|Default|Getfire1) false)
  (Components|Activation|Activate (Variables|Default|Getfire3) false))

(fn StopFire
  (Variables|Default|SetonFire false)
  (Components|Activation|Deactivate (Variables|Default|Getfire1))
  (Components|Activation|Deactivate (Variables|Default|Getfire2))
  (Components|Activation|Deactivate (Variables|Default|Getfire3)))

(fn GetNextSpawnPoint
  (bind _result (Math|Integer|IncrementInt (Variables|Default|GetspawnPointIndex))
    (:%20%20
      (if (> _result 4)
        (Variables|Default|SetspawnPointIndex 0))
      (switch int (Variables|Default|GetspawnPointIndex)
        (:Default
          _)
        (:0
          _)
        (:1
          (return (Variables|Default|GetspawnPoint2)))
        (:2
          (return (Variables|Default|GetspawnPoint3)))
        (:3
          (return (Variables|Default|GetspawnPoint4)))
        (:4
          (return (Variables|Default|GetspawnPoint5))))
      (return (Variables|Default|GetspawnPoint1)))))