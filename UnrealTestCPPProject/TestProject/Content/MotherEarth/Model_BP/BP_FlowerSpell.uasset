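; BP_FlowerSpell is a short-lived spell actor that spawns flowers on grass world tiles.
; On overlap with a grass WorldTileChild, it calls SpawnFlowers on that tile at its own location, then destroys itself.
; Otherwise it expires through a randomized countdown that drops once per Tick, so its lifetime depends on frame rate.
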(event Collision|EventActorBeginOverlap
  (params (OtherActor :type Actor%20Object%20Reference))
  (bind _asworld_tile_child (Utilities|Casting|CastToWorldTileChild OtherActor))
  (if (Variables|/Game/MotherEarth/WorldTileChild.WorldTileChild_C|GetIsGrass _asworld_tile_child)
    (Default|SpawnFlowers _asworld_tile_child (Transformation|GetActorLocation))
    (Actor|DestroyActor)))

(event EventTick
  (params (DeltaSeconds :type Float%20%28single-precision%29))
  (Variables|Default|SetdeathTimer (- (Variables|Default|GetdeathTimer) 1))
  (if (< (Variables|Default|GetdeathTimer) 0)
    (Actor|DestroyActor)))

(event EventBeginPlay
  (Variables|Default|SetdeathTimer (Math|Random|RandomIntegerinRange 40 70)))

(fn ConstructionScript)