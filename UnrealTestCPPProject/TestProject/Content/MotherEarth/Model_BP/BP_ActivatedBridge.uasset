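; BP_ActivatedBridge is a bridge actor that slides into place along the line running from the world origin through its position.
; MoveToStartingPosition offsets it toward the origin by StepSize times StepsAway.
; SummonBridge moves it outward one StepSize along the normalized position saved at BeginPlay, then SummonBridgeRecurse repeats this each tick via next-tick timers until CurrentStep equals StepsAway.
; Neither movement is triggered within this Blueprint.
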(event EventBeginPlay
  (Variables|Default|SetoriginalPosition (.location (Transformation|GetActorTransform))))

(fn ConstructionScript)

(fn SummonBridge
  (bind _returnvalue (Transformation|GetActorTransform))
  (bind _currentstep (Variables|Default|GetcurrentStep))
  (Transformation|SetActorTransform (Math|Transform|MakeTransform (+ (* (Math|Vector|Normalize (Variables|Default|GetoriginalPosition)) (Variables|Default|GetstepSize)) (.location _returnvalue)) (.rotation _returnvalue) (.scale _returnvalue)))
  (Math|Integer|IncrementInt _currentstep
    (:%20%20
      (if (not (== _currentstep (Variables|Default|GetstepsAway)))
        (Class|KismetSystemLibrary|SetTimerforNextTick 0 "SummonBridgeRecurse")))))

(fn SummonBridgeRecurse
  (bind _returnvalue (Transformation|GetActorTransform))
  (bind _currentstep (Variables|Default|GetcurrentStep))
  (Transformation|SetActorTransform (Math|Transform|MakeTransform (+ (* (Math|Vector|Normalize (Variables|Default|GetoriginalPosition)) (Variables|Default|GetstepSize)) (.location _returnvalue)) (.rotation _returnvalue) (.scale _returnvalue)))
  (Math|Integer|IncrementInt _currentstep
    (:%20%20
      (if (not (== _currentstep (Variables|Default|GetstepsAway)))
        (Class|KismetSystemLibrary|SetTimerforNextTick 0 "SummonBridgeRecurse")))))

(fn MovetoStartingPosition
  (Transformation|SetActorLocation (+ (* (Math|Vector|Normalize (- (Math|Vector|VectorZero) (Transformation|GetWorldLocation (Variables|Default|GetScene)))) (* (Variables|Default|GetstepSize) (Variables|Default|GetstepsAway))) (.location (Transformation|GetActorTransform))) false false))