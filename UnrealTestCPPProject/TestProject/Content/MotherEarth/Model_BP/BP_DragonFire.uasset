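; BP_DragonFire is a short-lived dragon fire actor that bursts into explosion chunks when it overlaps world tiles or characters.
; Tick decrements DeathTimer once per frame, so lifetime depends on frame rate, and destroys the actor silently when it runs out.
; Overlapping a land tile, water tile, player, minion or enemy spawns a batch of randomly oriented BP_FireExplosionChunk actors at its location, then destroys it.
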(event Collision|EventActorBeginOverlap
  (params (OtherActor :type Actor%20Object%20Reference))
  (bind _returnvalue (Transformation|GetActorLocation))
  (Utilities|Casting|CastToWorldTileChild OtherActor
    (:then
      _)
    (:CastFailed
      (Utilities|Casting|CastToWorldWaterTileChild OtherActor
        (:then
          _)
        (:CastFailed
          (Utilities|Casting|CastToGravityPlayerCharacter_BP OtherActor
            (:then
              _)
            (:CastFailed
              (Utilities|Casting|CastToGravityMinionCharacter_BP OtherActor
                (:then
                  _)
                (:CastFailed
                  (Utilities|Casting|CastToGravityEnemyCharacter_BP OtherActor)))))))))
  (for _index (range 0 10)
    (Game|SpawnActorfromClass "/Game/MotherEarth/Model_BP/BP_FireExplosionChunk.BP_FireExplosionChunk_C" (Math|Transform|MakeTransform _returnvalue (Math|Rotator|FindLookatRotation (Math|Vector|VectorZero) (* (Math|Random|RandomUnitVectorinConeinDegrees _returnvalue 1.8e+02) "1000.000000,1000.000000,1000.000000")) "1.000000,1.000000,1.000000") "Undefined" 0 0))
  (Actor|DestroyActor))

(event EventTick
  (params (DeltaSeconds :type Float%20%28single-precision%29))
  (Variables|Default|SetdeathTimer (- (Variables|Default|GetdeathTimer) 1))
  (if (< (Variables|Default|GetdeathTimer) 0)
    (Actor|DestroyActor)))

(fn ConstructionScript)