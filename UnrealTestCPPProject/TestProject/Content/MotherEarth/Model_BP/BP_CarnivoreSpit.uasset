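; BP_CarnivoreSpit is a spit actor that damages enemies it touches.
; On overlap with a GravityEnemyCharacter_BP, it applies its Damage value and destroys itself, ignoring other actors.
; Tick decrements DeathTimer by one per frame and destroys the actor once it drops below zero, so lifetime depends on frame rate.
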(event Collision|EventActorBeginOverlap
  (params (OtherActor :type Actor%20Object%20Reference))
  (bind _asgravity_enemy_character_bp (Utilities|Casting|CastToGravityEnemyCharacter_BP OtherActor))
  (Game|Damage|ApplyDamage _asgravity_enemy_character_bp (Variables|Default|Getdamage) 0 0)
  (Actor|DestroyActor))

(event EventTick
  (params (DeltaSeconds :type Float%20%28single-precision%29))
  (Variables|Default|SetdeathTimer (- (Variables|Default|GetdeathTimer) 1))
  (if (< (Variables|Default|GetdeathTimer) 0)
    (Actor|DestroyActor)))

(fn ConstructionScript)