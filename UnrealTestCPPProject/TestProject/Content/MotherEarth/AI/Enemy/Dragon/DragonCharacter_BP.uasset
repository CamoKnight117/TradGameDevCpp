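; Dragon enemy character that takes damage, heals, attacks through its AI controller and can be targeted by the player's selection.
; Damage and healing update a camera-facing health bar widget, and the actor is destroyed at zero health.
; Capsule overlaps start and end attacks on DragonAIControllerPlanet_BP, while Ctrl-click release outside marquee selection sets it as the selected units' enemy.
; Helpers set walk speed and point gravity through NinjaCharacterMovementComponent.
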(event OnComponentBeginOverlap(OverlapCapsuleComponent)
  (params (OverlappedComponent :type Primitive%20Component%20Object%20Reference) (OtherActor :type Actor%20Object%20Reference) (OtherComp :type Primitive%20Component%20Object%20Reference) (OtherBodyIndex :type Integer) (bFromSweep :type Boolean) (SweepResult :type Hit%20Result%20Structure%20%28by%20ref%29))
  ;[1 1 1] Detect overlaps and send request to controller to attack
  (bind _asdragon_aicontroller_planet_bp (Utilities|Casting|CastToDragonAIControllerPlanet_BP (Pawn|GetController)))
  (Default|TryAttackActor _asdragon_aicontroller_planet_bp OtherActor))

(event OnComponentEndOverlap(OverlapCapsuleComponent)
  (params (OverlappedComponent :type Primitive%20Component%20Object%20Reference) (OtherActor :type Actor%20Object%20Reference) (OtherComp :type Primitive%20Component%20Object%20Reference) (OtherBodyIndex :type Integer))
  ;[1 1 1] Detect overlaps and send request to controller to attack
  (bind _asdragon_aicontroller_planet_bp (Utilities|Casting|CastToDragonAIControllerPlanet_BP (Pawn|GetController)))
  (Default|EndAttack _asdragon_aicontroller_planet_bp OtherActor))

(event Custom|OnTakeAnyDamage_Event
  (params (DamagedActor :type Actor%20Object%20Reference) (Damage :type Float%20%28single-precision%29) (DamageType :type Damage%20Type%20Object%20Reference) (InstigatedBy :type Controller%20Object%20Reference) (DamageCauser :type Actor%20Object%20Reference))
  ;[1 1 1] Any Actor implementing the BP_HealthBar widget should ideally implement this code
  ;;[1 1 1] If damaged, decrease CurrentHealth and update the health bar, and destroy the actor if health less than 0
  (Rendering|SetVisibility (Variables|Default|GetHealthBar) true false)
  (bind _output_get (Variables|Default|SetCurrentHealth (- (Variables|Default|GetCurrentHealth) Damage)))
  (bind _asbp_enemy_health_bar (Utilities|Casting|CastToBP_EnemyHealthBar (UserInterface|GetWidget (Variables|Default|GetHealthBar))))
  (Default|SetHealth _asbp_enemy_health_bar (/ _output_get (Variables|Default|GetTotalHealth)))
  (if (<= (Variables|Default|GetCurrentHealth) 0.0)
    (Actor|DestroyActor)))

(event Custom|OnHealDamage
  (params (RestoredHealth :type Float%20%28double-precision%29))
  (bind _healthbar (Variables|Default|GetHealthBar))
  ;[1 1 1] Any Actor implementing the BP_HealthBar widget should ideally implement this code
  ;;[1 1 1] If healed, increase CurrentHealth and update the health bar, with max possible health being equal to TotalHealth
  (if (<= (+ RestoredHealth (Variables|Default|GetCurrentHealth)) (Variables|Default|GetTotalHealth))
    (Variables|Default|SetCurrentHealth (+ RestoredHealth (Variables|Default|GetCurrentHealth)))
    (else
      (Variables|Default|SetCurrentHealth (Variables|Default|GetTotalHealth))
      (Rendering|SetVisibility _healthbar false false)))
  (bind _asbp_enemy_health_bar (Utilities|Casting|CastToBP_EnemyHealthBar (UserInterface|GetWidget _healthbar)))
  (Default|SetHealth _asbp_enemy_health_bar (/ (Variables|Default|GetCurrentHealth) (Variables|Default|GetTotalHealth))))

(event EventTick
  (params (DeltaSeconds :type Float%20%28single-precision%29))
  (bind _returnvalue (Game|GetPlayerCameraManager 0))
  (bind _healthbar (Variables|Default|GetHealthBar))
  ;[1 1 1] Any Actor implementing the BP_HealthBar widget should ideally implement this code
  ;;[1 1 1] Keep the health bar rotated so the player can see it
  (Transformation|SetWorldRotation _healthbar (Math|Rotator|FindLookatRotation (Transformation|GetActorLocation (Game|Player|GetPlayerPawn 0)) (Camera|GetCameraLocation _returnvalue)) false false)
  (Transformation|AddRelativeRotation _healthbar (Class|KismetMathLibrary|NegateRotator (Math|Rotator|MakeRotator (.Roll (Math|Rotator|BreakRotator (Camera|GetCameraRotation _returnvalue))) 0.0 0.0)) false false))

(event EventActorOnReleased
  (params (ButtonReleased :type Key%20Structure :default "None"))
  ;[1 1 1] Targeting logic
  (bind _asgravity_player_controller_bp (Utilities|Casting|CastToGravityPlayerController_BP (Game|GetPlayerController 0)))
  (if (Variables|/Game/MotherEarth/GameObjects/GravityPlayerController_BP.GravityPlayerController_BP_C|GetleftCtrlPressed _asgravity_player_controller_bp)
    (bind _asme_hud (Utilities|Casting|CastToME_HUD (HUD|GetHUD _asgravity_player_controller_bp)))
    (if (not (Variables|/Game/MotherEarth/GameObjects/ME_HUD.ME_HUD_C|GetISMarquee _asme_hud))
      (Default|SetEnemyOfSelected _asgravity_player_controller_bp self))))

(event EventBeginPlay
  (Rendering|SetVisibility (Variables|Default|GetSelectionCircle) false false)
  (Rendering|SetVisibility (Variables|Default|GetHealthBar) false false)
  ;[1 1 1] Any Actor implementing the BP_HealthBar widget should ideally implement this code
  ;;[1 1 1] If damaged, decrease CurrentHealth and update the health bar, and destroy the actor if health less than 0
  (EventDispatchers|BindEventtoOnTakeAnyDamage (delegate Custom|OnTakeAnyDamage_Event))
  (Variables|Default|SetCurrentHealth (Variables|Default|GetTotalHealth)))

(fn ConstructionScript
  (|CallParentFunction))

(fn SetGravity
  (params (CenterOfGravity :type Vector))
  (bind _asninja_character_movement_component (Utilities|Casting|CastToNinjaCharacterMovementComponent (Variables|Character|GetCharacterMovement)))
  (Class|NinjaCharacterMovementComponent|SetPointGravityDirection _asninja_character_movement_component CenterOfGravity))

(fn UpdateWalkSpeed
  (params (NewWalkSpeed :type Float%20%28double-precision%29))
  (Variables|/Script/Engine.CharacterMovementComponent|SetMaxWalkSpeed (Variables|Character|GetCharacterMovement) NewWalkSpeed))