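; AI controller for enemies that runs BT_Enemy and steers pawns along async 3D paths from the CPath volume they overlap.
; Looping timers re-path and orient toward the next node, skipping ahead by velocity alignment and line traces, while Tick applies movement input.
; Perception and attack-overlap functions set blackboard targets and attack state.
; Helpers pick the nearest tree, or a reachable player-active StoneHenge base once enough regional enemies gather.
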(event OnTargetPerceptionUpdated(AIPerception)
  (params (Actor :type Actor%20Object%20Reference) (Stimulus :type AI%20Stimulus%20Structure))
  (bind _blackboard (Variables|Default|GetBlackboard))
  (bind _enemyactorkey (Variables|BlackboardKeys|GetEnemyActorKey))
  (if (or (Actor|ActorHasTag Actor (Variables|PerceptibleTags|GetPlayerTag)) (Actor|ActorHasTag Actor (Variables|PerceptibleTags|GetMinionTag)))
    (if (ScalableFloat|GetValueasBool (Variables|Default|GetBlackboard) (Variables|BlackboardKeys|GetIsAttackingKey))
      (Class|AIPerceptionComponent|ForgetAll (Variables|Default|GetAIPerception))
      (elif (Utilities|Struct|BreakAIStimulus Stimulus)
        (bind _volumeref (Variables|Pathfinding|GetVolumeRef)
          (:then
            (|FindPathAsync _volumeref (Transformation|GetActorLocation (Pawn|GetControlledPawn)) (Variables|Pathfinding|GetDestination) (Variables|GoToSettings|Additional|GetSmoothingPasses) 0.2
              (:Success
                (AI|Components|Blackboard|SetValueasObject _blackboard _enemyactorkey Actor)
                (AI|Components|Blackboard|SetValueasBool _blackboard (Variables|BlackboardKeys|GetIsAttackingKey) false))))
          (:else))
        (else
          (Utilities|FlowControl|RetriggerableDelay 0.3)
          (AI|Components|Blackboard|SetValueasObject _blackboard _enemyactorkey 0)
          (Class|AIPerceptionComponent|ForgetAll (Variables|Default|GetAIPerception)))))))

(event Custom|SetWaveAttackTarget
  (params (NumEnemiesRequired :type Integer))
  (Utilities|SetWaveAttackTargetCode NumEnemiesRequired))

(event Custom|CheckPath
  ;[1 1 1] Check and make the path - Recalculates path and stores results in PathBuffer and CurrentNodeIndex
  (if (Variables|Pathfinding|GetGoToRunning)
    (bind _volumeref (Variables|Pathfinding|GetVolumeRef)
      (:then
        (bind (_path _failreason) (|FindPathAsync _volumeref (Transformation|GetActorLocation (Pawn|GetControlledPawn)) (Variables|Pathfinding|GetDestination) (Variables|GoToSettings|Additional|GetSmoothingPasses) 0.2)
          (:Success
            (Variables|Pathfinding|SetPathBuffer _path)
            (bind _bestnodeindex (CallFunction|GetNextOptimalNode))
            (Variables|Pathfinding|SetCurrentNodeIndex _bestnodeindex))
          (:Failure
            (CallFunction|PauseMovement)
            (Variables|Pathfinding|SetDestination (Transformation|GetActorLocation (Pawn|GetControlledPawn)))
            (Class|AIPerceptionComponent|ForgetAll (Variables|Default|GetAIPerception)))))
      (:else))))

(event Custom|OrientToNextNode
  (bind _returnvalue (Pawn|GetControlledPawn))
  (bind _currentnodeindex (Variables|Pathfinding|GetCurrentNodeIndex))
  (bind _pathbuffer (Variables|Pathfinding|GetPathBuffer))
  (bind _returnvalue_2 (Transformation|GetActorLocation _returnvalue))
  (bind _output (Utilities|Array|Get(acopy) _pathbuffer _currentnodeindex))
  (bind _worldlocation (Utilities|Struct|BreakCPathNode _output))
  ;[1 1 1] Calculate CurrentInputVector and pawn's rotation based on the path in Path Buffer
  (if (Variables|Pathfinding|GetGoToRunning)
    (if (and (> (Math|Vector|Distance(Vector) _worldlocation _returnvalue_2) (Variables|GoToSettings|GetNodeDistanceTolerance)) (> (Math|Vector|Distance(Vector) (Variables|Pathfinding|GetDestination) _returnvalue_2) (Variables|Default|GetStoppingDistance))) :!label _label
      (Variables|Pathfinding|SetCurrentInputVector (Math|Vector|Normalize (- _worldlocation _returnvalue_2)))
      (Transformation|SetActorRotation (Pawn|GetControlledPawn) (Math|Interpolation|RInterpTo (Transformation|GetActorRotation (Pawn|GetControlledPawn)) (Math|Rotator|FindLookatRotation (Transformation|GetActorLocation (Pawn|GetControlledPawn)) _worldlocation) (Variables|GoToSettings|GetNodeDistanceCheckRate) 5.0))
      (else
        ;;[1 1 1] When end of Path Buffer reached, stop the overarching "Go To" cycle and set the input vector to zero
        (bind _result (Math|Integer|IncrementInt (Variables|Pathfinding|GetCurrentNodeIndex))
          (:%20%20
            (if (< _result (Utilities|Array|Length (Variables|Pathfinding|GetPathBuffer)))
              (goto _label)
              (else
                (CallFunction|PauseMovement)))))))))

(event EventBeginPlay
  (Class|AIPerceptionComponent|ForgetAll (Variables|Default|GetAIPerception))
  ;[1 1 1] Initialize variables and start the two custom events inside timer loops that make up the "Go To" cycle
  (Utilities|FlowControl|Delay 0.5)
  (Variables|PerceptibleTags|SetHostileList (Utilities|Array|MakeArray (Variables|PerceptibleTags|GetPlayerTag) (Variables|PerceptibleTags|GetMinionTag) (Variables|PerceptibleTags|GetTreeTag) (Variables|PerceptibleTags|GetBaseTag)))
  (Utilities|FlowControl|Sequence
    (:then_0
      (Variables|Pathfinding|SetCurrentNodeIndex 0)
      (bind _ascpath_volume (Utilities|Casting|CastToCPathVolume (Utilities|Array|Get(acopy) (Collision|GetOverlappingActors (Pawn|GetControlledPawn) "/Script/CPathfinding.CPathVolume" :!class /Script/Engine.Actor))))
      (Variables|Pathfinding|SetVolumeRef _ascpath_volume)
      (Utilities|FlowControl|Sequence
        (:then_0
          (if (> (Variables|GoToSettings|GetPath%20Recheck%20Rate) 0.0)
            (Utilities|Time|SetTimerbyEvent (delegate Custom|CheckPath) (Variables|GoToSettings|GetPath%20Recheck%20Rate) true)))
        (:then_1
          (Utilities|FlowControl|Delay 0.2)
          (Variables|Pathfinding|SetGoToRunning true)
          (Utilities|Time|SetTimerbyEvent (delegate Custom|OrientToNextNode) 0.2 true))))
    (:then_1
      (if (Variables|GoToSettings|Additional|GetDrawDebugPath)
        (Utilities|Time|SetTimerbyFunctionName 0 "DrawPath" 0.2 true)))))

(event EventTick
  (params (DeltaSeconds :type Float%20%28single-precision%29))
  ;[1 1 1] Add movement based on calculated path
  (Pawn|Input|AddMovementInput (Pawn|GetControlledPawn) (Variables|Pathfinding|GetCurrentInputVector) 1.0 false))

(event EventPossess
  (params (PossessedPawn :type Pawn%20Object%20Reference))
  (AI|RunBehaviorTree "/Game/MotherEarth/AI/Enemy/BT_Enemy.BT_Enemy"))

(fn ConstructionScript)

(fn GetDottoNode
  (params (Node :type C%20Path%20Node%20Structure))
  (return (Math|Vector|DotProduct (Math|Vector|Normalize (Variables|/Script/Engine.MovementComponent|GetVelocity (Pawn|GetMovementComponent (Pawn|GetControlledPawn)))) (Math|Vector|Normalize (- (.WorldLocation (Utilities|Struct|BreakCPathNode Node)) (Transformation|GetActorLocation (Pawn|GetControlledPawn)))))))

(fn GetNextOptimalNode
  (params (CurrentNodeIndex :type Integer))
  (LocalVariables|SetBestIndex CurrentNodeIndex)
  (LocalVariables|SetBestDot (CallFunction|GetDottoNode (Utilities|Array|Get(acopy) (Variables|Pathfinding|GetPathBuffer) CurrentNodeIndex)))
  (while (and (not (LocalVariables|GetWasHit)) (< (LocalVariables|GetBestIndex) (- (Utilities|Array|Length (Variables|Pathfinding|GetPathBuffer)) 1)))
    (bind _output_get (LocalVariables|SetCurrDot (CallFunction|GetDottoNode (Utilities|Array|Get(acopy) (Variables|Pathfinding|GetPathBuffer) (+ (LocalVariables|GetBestIndex) 1)))))
    (if (> _output_get (LocalVariables|GetBestDot))
      (bind _returnvalue (Collision|LineTraceByChannel (Transformation|GetActorLocation (Pawn|GetControlledPawn)) (.WorldLocation (Utilities|Struct|BreakCPathNode (Utilities|Array|Get(acopy) (Variables|Pathfinding|GetPathBuffer) (+ (LocalVariables|GetBestIndex) 1)))) "TraceTypeQuery1" false 0 "None"))
      (bind _output_get_2 (LocalVariables|SetWasHit _returnvalue))
      (if (not _output_get_2)
        (LocalVariables|SetBestDot (LocalVariables|GetCurrDot))
        (Math|Integer|IncrementInt (LocalVariables|GetBestIndex)
          (:%20%20
            (if (>= (LocalVariables|GetBestIndex) (- (Utilities|Array|Length (Variables|Pathfinding|GetPathBuffer)) 2))
              (return (LocalVariables|GetBestIndex))))))
      (else
        (return (LocalVariables|GetBestIndex)))))
  (return (LocalVariables|GetBestIndex)))

(fn DrawPath
  (if (and (Variables|GoToSettings|Additional|GetDrawDebugPath) (Utilities|IsValid (Variables|Pathfinding|GetVolumeRef)))
    (Class|CPathVolume|DrawDebugPath (Variables|Pathfinding|GetVolumeRef) (Variables|Pathfinding|GetPathBuffer) 0.2 true (Variables|GoToSettings|Additional|GetDebugPathColor))))

(fn UpdateDestination
  (params (Destination :type Vector))
  (if (Utilities|Operators|NotEqual(!=) Destination (Variables|Pathfinding|GetDestination) 5.0)
    (Variables|Pathfinding|SetDestination Destination)
    (Variables|Pathfinding|SetGoToRunning true)
    (CallFunction|CheckPath)
    (Pawn|SetControlRotation (Math|Rotator|FindLookatRotation (Transformation|GetActorLocation (Pawn|GetControlledPawn)) Destination))))

(fn TryAttackActor
  (params (AttackTarget :type Actor%20Object%20Reference))
  (bind _blackboard (Variables|Default|GetBlackboard))
  (bind _tagisvalid (CallFunction|HasValidAttackTag AttackTarget))
  (if _tagisvalid
    (Utilities|Set|Add (Variables|Default|GetOverlappingTargets) AttackTarget)
    (AI|Components|Blackboard|SetValueasObject _blackboard (Variables|BlackboardKeys|GetEnemyActorKey) AttackTarget)
    (AI|Components|Blackboard|SetValueasBool _blackboard (Variables|BlackboardKeys|GetIsAttackingKey) true)
    (CallFunction|PauseMovement)))

(fn HasValidAttackTag
  (params (Actor :type Actor%20Object%20Reference))
  (for _array_element (Variables|PerceptibleTags|GetHostileList)
    (LocalVariables|SetHasTagLocal (or (Actor|ActorHasTag Actor _array_element) (LocalVariables|GetHasTagLocal))))
  (return (LocalVariables|GetHasTagLocal)))

(fn EndAttack
  (params (AttackTarget :type Actor%20Object%20Reference))
  (bind _tagisvalid (CallFunction|HasValidAttackTag AttackTarget))
  (if _tagisvalid
    (bind _returnvalue (Utilities|Set|Remove (Variables|Default|GetOverlappingTargets) AttackTarget))
    (if _returnvalue
      (if (Utilities|Set|IsEmpty (Variables|Default|GetOverlappingTargets))
        (AI|Components|Blackboard|SetValueasBool (Variables|Default|GetBlackboard) (Variables|BlackboardKeys|GetIsAttackingKey) false)
        (AI|Components|Blackboard|SetValueasObject (Variables|Default|GetBlackboard) (Variables|BlackboardKeys|GetEnemyActorKey) 0)
        (Class|AIPerceptionComponent|ForgetAll (Variables|Default|GetAIPerception))
        (else
          (bind _result (Utilities|Set|ToArray (Variables|Default|GetOverlappingTargets)))
          (AI|Components|Blackboard|SetValueasObject (Variables|Default|GetBlackboard) (Variables|BlackboardKeys|GetEnemyActorKey) (Utilities|Array|Get(acopy) _result)))))))

(fn SetWaveAttackTarget
  (params (NumEnemiesRequired :type Integer))
  (bind _asbp_region_assigner (Utilities|Casting|CastToBP_regionAssigner (Utilities|Array|Get(acopy) (Collision|GetOverlappingActors (Pawn|GetControlledPawn) "/Game/MotherEarth/Model_BP/BP_regionAssigner.BP_regionAssigner_C" :!class /Script/Engine.Actor))))
  (if (>= (Utilities|Set|Length (Variables|/Game/MotherEarth/Model_BP/BP_regionAssigner.BP_regionAssigner_C|GetEnemyList _asbp_region_assigner)) NumEnemiesRequired)
    (bind _outactors (Actor|GetAllActorsOfClass "/Game/MotherEarth/Model_BP/BP_StoneHengeBase.BP_StoneHengeBase_C"))
    (bind _output_get (LocalVariables|SetBaseList _outactors))
    (if (Utilities|Array|IsEmpty _output_get) :!label _label
      (AI|Components|Blackboard|SetValueasObject (Variables|Default|GetBlackboard) (Variables|BlackboardKeys|GetBaseActorKey) 0)
      (return false)
      (else
        (bind _asbp_stone_henge_base (Utilities|Casting|CastToBP_StoneHengeBase (.ReturnValue (Actor|FindNearestActor (Transformation|GetActorLocation (Pawn|GetControlledPawn)) _output_get))))
        (if (Variables|/Game/MotherEarth/Model_BP/BP_StoneHengeBase.BP_StoneHengeBase_C|GetenemyActive _asbp_stone_henge_base)
          (Utilities|Array|RemoveItem (LocalVariables|GetBaseList) _asbp_stone_henge_base)
          (goto _label)
          (else
            (AI|Components|Blackboard|SetValueasObject (Variables|Default|GetBlackboard) (Variables|BlackboardKeys|GetBaseActorKey) _asbp_stone_henge_base)
            (return true)))))))

(fn SetClosestTree
  (bind _treeactorkey (Variables|BlackboardKeys|GetTreeActorKey))
  (bind _blackboard (Variables|Default|GetBlackboard))
  (bind _outactors (Actor|GetAllActorsOfClass "/Game/MotherEarth/Model_BP/BP_Tree.BP_Tree_C"))
  (if (Utilities|Array|IsEmpty _outactors)
    _
    (elif (>= (.Distance (Actor|FindNearestActor (Transformation|GetActorLocation (Pawn|GetControlledPawn)) _outactors)) (Variables|Default|GetTreeSightDistance))
      _
      (else
        (AI|Components|Blackboard|SetValueasObject _blackboard _treeactorkey (.ReturnValue (Actor|FindNearestActor (Transformation|GetActorLocation (Pawn|GetControlledPawn)) _outactors)))
        (return true))))
  (AI|Components|Blackboard|SetValueasObject _blackboard _treeactorkey 0)
  (return false))

(fn PauseMovement
  (Variables|Pathfinding|SetGoToRunning false)
  (Variables|Pathfinding|SetCurrentInputVector "0, 0, 0"))

(fn ResumeMovement
  (Variables|Pathfinding|SetGoToRunning true))