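; Player-selectable allied minion character that supports point gravity through Ninja character movement.
; Click and Shift-click update the player controller's selection, which toggles circles on the minion and its target.
; Capsule overlaps feed its AI controller, setting the blackboard region (sight perception off inside) or starting and ending attacks.
; Damage and timed healing from counted flower overlaps drive a camera-facing health bar; death updates the home base's count and the selection.
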(event OnComponentBeginOverlap(OverlapCapsuleComponent)
  (params (OverlappedComponent :type Primitive%20Component%20Object%20Reference) (OtherActor :type Actor%20Object%20Reference) (OtherComp :type Primitive%20Component%20Object%20Reference) (OtherBodyIndex :type Integer) (bFromSweep :type Boolean) (SweepResult :type Hit%20Result%20Structure%20%28by%20ref%29))
  (bind _asminion_aicontroller_planet_bp (Utilities|Casting|CastToMinionAIControllerPlanet_BP (Pawn|GetController)))
  ;[1 1 1] If overlapping with a BP_RegionBounds, set it as this minion's region
  (bind _asbp_region_bounds (Utilities|Casting|CastToBP_RegionBounds OtherActor)
    (:then
      (AI|Components|Blackboard|SetValueasObject (Variables|/Script/AIModule.AIController|GetBlackboard _asminion_aicontroller_planet_bp) (Variables|Default|GetRegionBoundsKey) _asbp_region_bounds)
      (Class|AIPerceptionComponent|SetSenseEnabled (Variables|/Game/MotherEarth/AI/Minion/MinionAIControllerPlanet_BP.MinionAIControllerPlanet_BP_C|GetAIPerception _asminion_aicontroller_planet_bp) "/Script/AIModule.AISense_Sight" false)
      (Class|AIPerceptionComponent|ForgetAll (Variables|/Game/MotherEarth/AI/Minion/MinionAIControllerPlanet_BP.MinionAIControllerPlanet_BP_C|GetAIPerception _asminion_aicontroller_planet_bp)))
    (:CastFailed
      ;[1 1 1] Otherwise, try to attack it
      (Default|TryAttackActor _asminion_aicontroller_planet_bp OtherActor))))

(event OnComponentEndOverlap(OverlapCapsuleComponent)
  (params (OverlappedComponent :type Primitive%20Component%20Object%20Reference) (OtherActor :type Actor%20Object%20Reference) (OtherComp :type Primitive%20Component%20Object%20Reference) (OtherBodyIndex :type Integer))
  (bind _asminion_aicontroller_planet_bp (Utilities|Casting|CastToMinionAIControllerPlanet_BP (Pawn|GetController)))
  ;[1 1 1] If no longer overlapping the region set as this minion's region, remove the reference to it
  (bind _asbp_region_bounds (Utilities|Casting|CastToBP_RegionBounds OtherActor)
    (:then
      (if (== _asbp_region_bounds (AI|Components|Blackboard|GetValueasObject (Variables|/Script/AIModule.AIController|GetBlackboard _asminion_aicontroller_planet_bp) (Variables|Default|GetRegionBoundsKey)))
        (AI|Components|Blackboard|SetValueasObject (Variables|/Script/AIModule.AIController|GetBlackboard _asminion_aicontroller_planet_bp) (Variables|Default|GetRegionBoundsKey) 0)
        (Class|AIPerceptionComponent|SetSenseEnabled (Variables|/Game/MotherEarth/AI/Minion/MinionAIControllerPlanet_BP.MinionAIControllerPlanet_BP_C|GetAIPerception _asminion_aicontroller_planet_bp) "/Script/AIModule.AISense_Sight" true)))
    (:CastFailed
      (Default|EndAttack _asminion_aicontroller_planet_bp OtherActor))))

(event Custom|ISSelected
  (params (IsSelected :type Boolean))
  ;[1 1 1] Allows Minions to be selectable
  (bind _output_get (Variables|Default|SetSelected IsSelected))
  (Rendering|SetVisibility (Variables|Default|GetSelectionCircle) _output_get false)
  (if _output_get
    (CallFunction|UpdateSelectionTarget (Variables|Default|GetCurrentTarget))
    (else
      (bind _asgravity_player_controller_bp (Utilities|Casting|CastToGravityPlayerController_BP (Game|GetPlayerController 0)))
      (bind _hastarget (Default|HasSelectedTarget _asgravity_player_controller_bp (Variables|Default|GetCurrentTarget) self))
      (if (not _hastarget)
        (CallFunction|ClearSelectionTarget)))))

(event Custom|OnTakeAnyDamage_Event
  (params (DamagedActor :type Actor%20Object%20Reference) (Damage :type Float%20%28single-precision%29) (DamageType :type Damage%20Type%20Object%20Reference) (InstigatedBy :type Controller%20Object%20Reference) (DamageCauser :type Actor%20Object%20Reference))
  (bind _homebase (Variables|Default|GethomeBase))
  ;[1 1 1] Any Actor implementing the BP_HealthBar widget should ideally implement this code
  ;;[1 1 1] If damaged, decrease CurrentHealth and update the health bar, and destroy the actor if health less than 0
  (Rendering|SetVisibility (Variables|Default|GetHealthBar) true false)
  (bind _output_get (Variables|Default|SetCurrentHealth (- (Variables|Default|GetCurrentHealth) Damage)))
  (bind _asbp_ally_health_bar (Utilities|Casting|CastToBP_AllyHealthBar (UserInterface|GetWidget (Variables|Default|GetHealthBar))))
  (Default|SetHealth _asbp_ally_health_bar (/ _output_get (Variables|Default|GetTotalHealth)))
  (if (<= (Variables|Default|GetCurrentHealth) 0.0)
    (Utilities|IsValid _homebase
      (:Is%20Valid
        (Variables|/Game/MotherEarth/Model_BP/BP_StoneHengeBase.BP_StoneHengeBase_C|SetminionsSpawned _homebase (- (Variables|/Game/MotherEarth/Model_BP/BP_StoneHengeBase.BP_StoneHengeBase_C|GetminionsSpawned _homebase) 1)))
      (:Is%20Not%20Valid
        _))
    (bind _asgravity_player_controller_bp (Utilities|Casting|CastToGravityPlayerController_BP (Game|GetPlayerController 0)))
    (Default|RemoveUnitfromSelection _asgravity_player_controller_bp self)
    (Actor|DestroyActor)))

(event Custom|OnHealDamage
  (params (RestoredHealth :type Float%20%28double-precision%29))
  (bind _healthbar (Variables|Default|GetHealthBar))
  ;[1 1 1] Any Actor implementing the BP_HealthBar widget should ideally implement this code
  ;;[1 1 1] If healed, increase CurrentHealth and update the health bar, with max possible health being equal to TotalHealth
  (if (<= (+ RestoredHealth (Variables|Default|GetCurrentHealth)) (Variables|Default|GetTotalHealth))
    (Variables|Default|SetCurrentHealth (+ RestoredHealth (Variables|Default|GetCurrentHealth)))
    (else
      (Variables|Default|SetCurrentHealth (Variables|Default|GetTotalHealth))
      (Rendering|SetVisibility _healthbar false false)))
  (bind _asbp_ally_health_bar (Utilities|Casting|CastToBP_AllyHealthBar (UserInterface|GetWidget _healthbar)))
  (Default|SetHealth _asbp_ally_health_bar (/ (Variables|Default|GetCurrentHealth) (Variables|Default|GetTotalHealth))))

(event EventPossessed
  (params (NewController :type Controller%20Object%20Reference)))

(event EventTick
  (params (DeltaSeconds :type Float%20%28single-precision%29))
  (bind _returnvalue (Game|GetPlayerCameraManager 0))
  (bind _healthbar (Variables|Default|GetHealthBar))
  ;[1 1 1] Any Actor implementing the BP_HealthBar widget should ideally implement this code
  ;;[1 1 1] Keep the health bar rotated so the player can see it
  (Transformation|SetWorldRotation _healthbar (Math|Rotator|FindLookatRotation (Transformation|GetActorLocation (Game|Player|GetPlayerPawn 0)) (Camera|GetCameraLocation _returnvalue)) false false)
  (Transformation|AddRelativeRotation _healthbar (Class|KismetMathLibrary|NegateRotator (Math|Rotator|MakeRotator (.Roll (Math|Rotator|BreakRotator (Camera|GetCameraRotation _returnvalue))) 0.0 0.0)) false false))

(event MouseInput|EventActorOnClicked
  (params (ButtonPressed :type Key%20Structure))
  ;[1 1 1] Allows Minions to be selectable
  (if (== ButtonPressed "LeftMouseButton")
    (bind _asgravity_player_controller_bp (Utilities|Casting|CastToGravityPlayerController_BP (Game|GetPlayerController 0)))
    (if (Variables|/Game/MotherEarth/GameObjects/GravityPlayerController_BP.GravityPlayerController_BP_C|GetleftShiftPressed _asgravity_player_controller_bp)
      (if (Variables|Default|GetSelected)
        (Default|RemoveUnitfromSelection _asgravity_player_controller_bp self :!label _label)
        (else
          (Default|AddUnittoSelection _asgravity_player_controller_bp self :!label _label_2)))
      (elif (and (Variables|Default|GetSelected) (== (Utilities|Array|Length (Variables|/Game/MotherEarth/GameObjects/GravityPlayerController_BP.GravityPlayerController_BP_C|GetMinionSelection _asgravity_player_controller_bp)) 1))
        (goto _label)
        (else
          (Default|ClearUnitSelection _asgravity_player_controller_bp)
          (goto _label_2))))))

(event EventBeginPlay
  (bind _overlappingactors (Collision|GetOverlappingActors "/Game/MotherEarth/GameObjects/BP_RegionBounds.BP_RegionBounds_C" :!class /Script/Engine.Actor))
  (Rendering|SetVisibility (Variables|Default|GetSelectionCircle) false false)
  (Rendering|SetVisibility (Variables|Default|GetHealthBar) false false)
  (bind _returnvalue (Actor|GetActorOfClass "/Game/MotherEarth/GameObjects/GravityBounds_BP.GravityBounds_BP_C"))
  (Default|UpdateGravityFunc _returnvalue)
  (bind _asminion_aicontroller_planet_bp (Utilities|Casting|CastToMinionAIControllerPlanet_BP (Pawn|GetController)))
  (Variables|/Game/MotherEarth/AI/Minion/MinionAIControllerPlanet_BP.MinionAIControllerPlanet_BP_C|SetDestination _asminion_aicontroller_planet_bp (Transformation|GetActorLocation))
  (AI|Components|Blackboard|SetValueasObject (Variables|/Script/AIModule.AIController|GetBlackboard _asminion_aicontroller_planet_bp) (Variables|Default|GetRegionBoundsKey) (Utilities|Array|Get(acopy) _overlappingactors))
  (if (Utilities|Array|IsEmpty _overlappingactors)
    (Class|AIPerceptionComponent|SetSenseEnabled (Variables|/Game/MotherEarth/AI/Minion/MinionAIControllerPlanet_BP.MinionAIControllerPlanet_BP_C|GetAIPerception _asminion_aicontroller_planet_bp) "/Script/AIModule.AISense_Sight" true))
  ;[1 1 1] Any Actor implementing the BP_HealthBar widget should ideally implement this code
  ;;[1 1 1] If damaged, decrease CurrentHealth and update the health bar, and destroy the actor if health less than 0
  (EventDispatchers|BindEventtoOnTakeAnyDamage (delegate Custom|OnTakeAnyDamage_Event))
  (Variables|Default|SetCurrentHealth (Variables|Default|GetTotalHealth)))

(fn ConstructionScript
  (|CallParentFunction))

(fn SetGravity
  (params (CenterOfGravity :type Vector))
  (bind _asninja_character_movement_component (Utilities|Casting|CastToNinjaCharacterMovementComponent (Variables|Character|GetCharacterMovement)))
  (Class|NinjaCharacterMovementComponent|SetPointGravityDirection _asninja_character_movement_component CenterOfGravity))

(fn UpdateWalkSpeed
  (params (NewWalkSpeed :type Float%20%28double-precision%29))
  (Variables|/Script/Engine.CharacterMovementComponent|SetMaxWalkSpeed (Variables|Character|GetCharacterMovement) NewWalkSpeed))

(fn StartHealing
  (if (not (Variables|Default|Gethealing))
    (Components|Activation|Activate (Variables|Default|GethealingParticleSystem) false)
    (Utilities|Time|SetTimerbyFunctionName 0 "continueHealing" 1.0)
    (Variables|Default|Sethealing true)))

(fn ContinueHealing
  (if (Variables|Default|Gethealing)
    (Utilities|Time|SetTimerbyFunctionName 0 "continueHealing" 1.0)
    (CallFunction|OnHealDamage (Variables|Default|GethealRate))
    (else
      (CallFunction|StopHealing))))

(fn StopHealing
  (Components|Activation|Deactivate (Variables|Default|GethealingParticleSystem))
  (Variables|Default|Sethealing false))

(fn AddtoFlowerOverlap
  (bind _totalfloweroverlap (Variables|Default|GettotalFlowerOverlap))
  (Math|Integer|IncrementInt _totalfloweroverlap
    (:%20%20
      (if (== _totalfloweroverlap 1)
        (CallFunction|StartHealing)))))

(fn RemovefromFlowerOverlap
  (bind _totalfloweroverlap (Variables|Default|GettotalFlowerOverlap))
  (Math|Integer|DecrementInt _totalfloweroverlap
    (:%20%20
      (if (<= _totalfloweroverlap 0)
        (CallFunction|StopHealing)))))

(fn ClearSelectionTarget
  (bind _currenttarget (Variables|Default|GetCurrentTarget))
  (Utilities|IsValid _currenttarget
    (:Is%20Valid
      (bind _asgravity_player_character_bp (Utilities|Casting|CastToGravityPlayerCharacter_BP _currenttarget)
        (:then
          (Rendering|SetVisibility (Variables|/Game/MotherEarth/GravityPlayerCharacter_BP.GravityPlayerCharacter_BP_C|GetSelectionCircle _asgravity_player_character_bp) false false))
        (:CastFailed
          (bind _asgravity_enemy_character_bp (Utilities|Casting|CastToGravityEnemyCharacter_BP _currenttarget)
            (:then
              (Rendering|SetVisibility (Variables|/Game/MotherEarth/AI/Enemy/GravityEnemyCharacter_BP.GravityEnemyCharacter_BP_C|GetSelectionCircle _asgravity_enemy_character_bp) false false))
            (:CastFailed
              (bind _asbp_crystal (Utilities|Casting|CastToBP_Crystal _currenttarget)
                (:then
                  (Rendering|SetVisibility (Variables|/Game/MotherEarth/Model_BP/BP_Crystal.BP_Crystal_C|GetSelectionCircle _asbp_crystal) false false))
                (:CastFailed
                  (bind _asbp_dragon (Utilities|Casting|CastToBP_Dragon _currenttarget))
                  (Rendering|SetVisibility (Variables|/Game/MotherEarth/Model_BP/BP_Dragon.BP_Dragon_C|GetSelectionCircle _asbp_dragon) false false))))))))))

(fn UpdateSelectionTarget
  (params (NewTarget :type Actor%20Object%20Reference))
  (if (== NewTarget (Variables|Default|GetCurrentTarget))
    _
    (else
      (CallFunction|ClearSelectionTarget)))
  (Utilities|IsValid NewTarget
    (:Is%20Valid
      (bind _asgravity_player_character_bp (Utilities|Casting|CastToGravityPlayerCharacter_BP NewTarget)
        (:then
          (Variables|Default|SetCurrentTarget _asgravity_player_character_bp)
          (if (Variables|Default|GetSelected)
            (Rendering|SetVisibility (Variables|/Game/MotherEarth/GravityPlayerCharacter_BP.GravityPlayerCharacter_BP_C|GetSelectionCircle _asgravity_player_character_bp) true false)))
        (:CastFailed
          (bind _asgravity_enemy_character_bp (Utilities|Casting|CastToGravityEnemyCharacter_BP NewTarget)
            (:then
              (Variables|Default|SetCurrentTarget _asgravity_enemy_character_bp)
              (if (Variables|Default|GetSelected)
                (Rendering|SetVisibility (Variables|/Game/MotherEarth/AI/Enemy/GravityEnemyCharacter_BP.GravityEnemyCharacter_BP_C|GetSelectionCircle _asgravity_enemy_character_bp) true false)))
            (:CastFailed
              (bind _asbp_crystal (Utilities|Casting|CastToBP_Crystal NewTarget)
                (:then
                  (Variables|Default|SetCurrentTarget _asbp_crystal)
                  (if (Variables|Default|GetSelected)
                    (Rendering|SetVisibility (Variables|/Game/MotherEarth/Model_BP/BP_Crystal.BP_Crystal_C|GetSelectionCircle _asbp_crystal) true false)))
                (:CastFailed
                  (bind _asbp_dragon (Utilities|Casting|CastToBP_Dragon NewTarget))
                  (Variables|Default|SetCurrentTarget _asbp_dragon)
                  (if (Variables|Default|GetSelected)
                    (Rendering|SetVisibility (Variables|/Game/MotherEarth/Model_BP/BP_Dragon.BP_Dragon_C|GetSelectionCircle _asbp_dragon) true false)))))))))))