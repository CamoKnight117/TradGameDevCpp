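; Selectable allied plant minion character that tracks health, destroys itself at zero and billboards its ally health bar toward the camera.
; Capsule overlaps tell its DragonAIControllerPlanet_BP to start or end attacks, and Ninja character movement supports point gravity.
; A flower overlap counter drives a looping one-second heal timer with particles.
; Target updates toggle selection circles on players, enemies or crystals, showing them only while the minion is selected.
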(event OnComponentBeginOverlap(OverlapCapsuleComponent)
  (params (OverlappedComponent :type Primitive%20Component%20Object%20Reference) (OtherActor :type Actor%20Object%20Reference) (OtherComp :type Primitive%20Component%20Object%20Reference) (OtherBodyIndex :type Integer) (bFromSweep :type Boolean) (SweepResult :type Hit%20Result%20Structure%20%28by%20ref%29))
  ;[1 1 1] Detect overlaps and send request to controller to attack
  (bind _asdragon_aicontroller_planet_bp (Utilities|Casting|CastToDragonAIControllerPlanet_BP (Pawn|GetController)))
  (Default|TryAttackActor _asdragon_aicontroller_planet_bp OtherActor))

(event OnComponentEndOverlap(OverlapCapsuleComponent)
  (params (OverlappedComponent :type Primitive%20Component%20Object%20Reference) (OtherActor :type Actor%20Object%20Reference) (OtherComp :type Primitive%20Component%20Object%20Reference) (OtherBodyIndex :type Integer))
  ;[1 1 1] Detect overlaps and send request to controller to attack
  (bind _asdragon_aicontroller_planet_bp (Utilities|Casting|CastToDragonAIControllerPlanet_BP (Pawn|GetController)))
  (Default|EndAttack _asdragon_aicontroller_planet_bp OtherActor))

(event Custom|OnTakeAnyDamage_Event
  (params (DamagedActor :type Actor%20Object%20Reference) (Damage :type Float%20%28single-precision%29) (DamageType :type Damage%20Type%20Object%20Reference) (InstigatedBy :type Controller%20Object%20Reference) (DamageCauser :type Actor%20Object%20Reference))
  ;[1 1 1] Any Actor implementing the BP_HealthBar widget should ideally implement this code
  ;;[1 1 1] If damaged, decrease CurrentHealth and update the health bar, and destroy the actor if health less than 0
  (Rendering|SetVisibility (Variables|Default|GetHealthBar) true false)
  (bind _output_get (Variables|Default|SetCurrentHealth (- (Variables|Default|GetCurrentHealth) Damage)))
  (bind _asbp_ally_health_bar (Utilities|Casting|CastToBP_AllyHealthBar (UserInterface|GetWidget (Variables|Default|GetHealthBar))))
  (Default|SetHealth _asbp_ally_health_bar (/ _output_get (Variables|Default|GetTotalHealth)))
  (if (<= (Variables|Default|GetCurrentHealth) 0.0)
    (Actor|DestroyActor)))

(event Custom|OnHealDamage
  (params (RestoredHealth :type Float%20%28double-precision%29))
  (bind _healthbar (Variables|Default|GetHealthBar))
  ;[1 1 1] Any Actor implementing the BP_HealthBar widget should ideally implement this code
  ;;[1 1 1] If healed, increase CurrentHealth and update the health bar, with max possible health being equal to TotalHealth
  (if (<= (+ RestoredHealth (Variables|Default|GetCurrentHealth)) (Variables|Default|GetTotalHealth))
    (Variables|Default|SetCurrentHealth (+ RestoredHealth (Variables|Default|GetCurrentHealth)))
    (else
      (Variables|Default|SetCurrentHealth (Variables|Default|GetTotalHealth))
      (Rendering|SetVisibility _healthbar false false)))
  (bind _asbp_ally_health_bar (Utilities|Casting|CastToBP_AllyHealthBar (UserInterface|GetWidget _healthbar)))
  (Default|SetHealth _asbp_ally_health_bar (/ (Variables|Default|GetCurrentHealth) (Variables|Default|GetTotalHealth))))

(event EventTick
  (params (DeltaSeconds :type Float%20%28single-precision%29))
  (bind _returnvalue (Game|GetPlayerCameraManager 0))
  (bind _healthbar (Variables|Default|GetHealthBar))
  ;[1 1 1] Any Actor implementing the BP_HealthBar widget should ideally implement this code
  ;;[1 1 1] Keep the health bar rotated so the player can see it
  (Transformation|SetWorldRotation _healthbar (Math|Rotator|FindLookatRotation (Transformation|GetActorLocation (Game|Player|GetPlayerPawn 0)) (Camera|GetCameraLocation _returnvalue)) false false)
  (Transformation|AddRelativeRotation _healthbar (Class|KismetMathLibrary|NegateRotator (Math|Rotator|MakeRotator (.Roll (Math|Rotator|BreakRotator (Camera|GetCameraRotation _returnvalue))) 0.0 0.0)) false false))

(event EventBeginPlay
  (Rendering|SetVisibility (Variables|Default|GetSelectionCircle) false false)
  (Rendering|SetVisibility (Variables|Default|GetHealthBar) false false)
  ;[1 1 1] Any Actor implementing the BP_HealthBar widget should ideally implement this code
  ;;[1 1 1] If damaged, decrease CurrentHealth and update the health bar, and destroy the actor if health less than 0
  (EventDispatchers|BindEventtoOnTakeAnyDamage (delegate Custom|OnTakeAnyDamage_Event))
  (Variables|Default|SetCurrentHealth (Variables|Default|GetTotalHealth)))

(fn ConstructionScript
  (|CallParentFunction))

(fn SetGravity
  (params (CenterOfGravity :type Vector))
  (bind _asninja_character_movement_component (Utilities|Casting|CastToNinjaCharacterMovementComponent (Variables|Character|GetCharacterMovement)))
  (Class|NinjaCharacterMovementComponent|SetPointGravityDirection _asninja_character_movement_component CenterOfGravity))

(fn UpdateWalkSpeed
  (params (NewWalkSpeed :type Float%20%28double-precision%29))
  (Variables|/Script/Engine.CharacterMovementComponent|SetMaxWalkSpeed (Variables|Character|GetCharacterMovement) NewWalkSpeed))

(fn StartHealing
  (if (not (Variables|Default|Gethealing))
    (Components|Activation|Activate (Variables|Default|GethealingParticleSystem) false)
    (Utilities|Time|SetTimerbyFunctionName 0 "continueHealing" 1.0)
    (Variables|Default|Sethealing true)))

(fn ContinueHealing
  (if (Variables|Default|Gethealing)
    (Utilities|Time|SetTimerbyFunctionName 0 "continueHealing" 1.0)
    (CallFunction|OnHealDamage (Variables|Default|GethealRate))
    (else
      (CallFunction|StopHealing))))

(fn StopHealing
  (Components|Activation|Deactivate (Variables|Default|GethealingParticleSystem))
  (Variables|Default|Sethealing false))

(fn AddtoFlowerOverlap
  (bind _totalfloweroverlap (Variables|Default|GettotalFlowerOverlap))
  (Math|Integer|IncrementInt _totalfloweroverlap
    (:%20%20
      (if (== _totalfloweroverlap 1)
        (CallFunction|StartHealing)))))

(fn RemovefromFlowerOverlap
  (bind _totalfloweroverlap (Variables|Default|GettotalFlowerOverlap))
  (Math|Integer|DecrementInt _totalfloweroverlap
    (:%20%20
      (if (<= _totalfloweroverlap 0)
        (CallFunction|StopHealing)))))

(fn ClearSelectionTarget
  (bind _currenttarget (Variables|Default|GetCurrentTarget))
  (Utilities|IsValid _currenttarget
    (:Is%20Valid
      (bind _asgravity_player_character_bp (Utilities|Casting|CastToGravityPlayerCharacter_BP _currenttarget)
        (:then
          (Rendering|SetVisibility (Variables|/Game/MotherEarth/GravityPlayerCharacter_BP.GravityPlayerCharacter_BP_C|GetSelectionCircle _asgravity_player_character_bp) false false))
        (:CastFailed
          (bind _asgravity_enemy_character_bp (Utilities|Casting|CastToGravityEnemyCharacter_BP _currenttarget)
            (:then
              (Rendering|SetVisibility (Variables|/Game/MotherEarth/AI/Enemy/GravityEnemyCharacter_BP.GravityEnemyCharacter_BP_C|GetSelectionCircle _asgravity_enemy_character_bp) false false))
            (:CastFailed
              (bind _asbp_crystal (Utilities|Casting|CastToBP_Crystal _currenttarget))
              (Rendering|SetVisibility (Variables|/Game/MotherEarth/Model_BP/BP_Crystal.BP_Crystal_C|GetSelectionCircle _asbp_crystal) false false))))))))

(fn UpdateSelectionTarget
  (params (NewTarget :type Actor%20Object%20Reference))
  (if (== NewTarget (Variables|Default|GetCurrentTarget))
    _
    (else
      (CallFunction|ClearSelectionTarget)))
  (Utilities|IsValid NewTarget
    (:Is%20Valid
      (bind _asgravity_player_character_bp (Utilities|Casting|CastToGravityPlayerCharacter_BP NewTarget)
        (:then
          (Variables|Default|SetCurrentTarget _asgravity_player_character_bp)
          (if (Variables|Default|GetSelected)
            (Rendering|SetVisibility (Variables|/Game/MotherEarth/GravityPlayerCharacter_BP.GravityPlayerCharacter_BP_C|GetSelectionCircle _asgravity_player_character_bp) true false)))
        (:CastFailed
          (bind _asgravity_enemy_character_bp (Utilities|Casting|CastToGravityEnemyCharacter_BP NewTarget)
            (:then
              (Variables|Default|SetCurrentTarget _asgravity_enemy_character_bp)
              (if (Variables|Default|GetSelected)
                (Rendering|SetVisibility (Variables|/Game/MotherEarth/AI/Enemy/GravityEnemyCharacter_BP.GravityEnemyCharacter_BP_C|GetSelectionCircle _asgravity_enemy_character_bp) true false)))
            (:CastFailed
              (bind _asbp_crystal (Utilities|Casting|CastToBP_Crystal NewTarget))
              (Variables|Default|SetCurrentTarget _asbp_crystal)
              (if (Variables|Default|GetSelected)
                (Rendering|SetVisibility (Variables|/Game/MotherEarth/Model_BP/BP_Crystal.BP_Crystal_C|GetSelectionCircle _asbp_crystal) true false)))))))))