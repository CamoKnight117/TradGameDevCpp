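; AI controller for a plant minion that runs BT_Plant and supplies its blackboard with an enemy target.
; Sight perception sets the target from tagged enemies, clearing it and forgetting all after a short retriggerable delay when sight is lost.
; TryAttackActor and EndAttack track hostile-tagged targets in an overlap set, setting a touching flag that overrides sight updates.
; EndAttack retargets to a remaining overlap, or resets target, flag and perception when none remain.
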(event OnTargetPerceptionUpdated(AIPerception)
  (params (Actor :type Actor%20Object%20Reference) (Stimulus :type AI%20Stimulus%20Structure))
  (bind _blackboard (Variables|Default|GetBlackboard))
  (bind _enemyactorkey (Variables|BlackboardKeys|GetEnemyActorKey))
  (if (Actor|ActorHasTag Actor (Variables|PerceptibleTags|GetEnemyTag))
    (if (ScalableFloat|GetValueasBool (Variables|Default|GetBlackboard) (Variables|BlackboardKeys|GetIsTouchingKey))
      (Class|AIPerceptionComponent|ForgetAll (Variables|Default|GetAIPerception))
      (elif (Utilities|Struct|BreakAIStimulus Stimulus)
        (AI|Components|Blackboard|SetValueasObject _blackboard _enemyactorkey Actor)
        (else
          (Utilities|FlowControl|RetriggerableDelay 0.3)
          (AI|Components|Blackboard|SetValueasObject _blackboard _enemyactorkey 0)
          (Class|AIPerceptionComponent|ForgetAll (Variables|Default|GetAIPerception)))))))

(event EventBeginPlay
  (Utilities|FlowControl|Delay 0.5)
  (Class|AIPerceptionComponent|SetSenseEnabled (Variables|Default|GetAIPerception) "/Script/AIModule.AISense_Sight" true)
  (Class|AIPerceptionComponent|ForgetAll (Variables|Default|GetAIPerception))
  (Utilities|FlowControl|Delay 0.5)
  (Variables|PerceptibleTags|SetHostileList (Utilities|Array|MakeArray (Variables|PerceptibleTags|GetEnemyTag))))

(event EventTick
  (params (DeltaSeconds :type Float%20%28single-precision%29)))

(event EventPossess
  (params (PossessedPawn :type Pawn%20Object%20Reference))
  (AI|RunBehaviorTree "/Game/MotherEarth/AI/Minion/Plant/BT_Plant.BT_Plant"))

(fn ConstructionScript)

(fn TryAttackActor
  (params (AttackTarget :type Actor%20Object%20Reference))
  (bind _blackboard (Variables|Default|GetBlackboard))
  (bind _tagisvalid (CallFunction|HasValidAttackTag AttackTarget))
  (if _tagisvalid
    (Utilities|Set|Add (Variables|Default|GetOverlappingTargets) AttackTarget)
    (AI|Components|Blackboard|SetValueasObject _blackboard (Variables|BlackboardKeys|GetEnemyActorKey) AttackTarget)
    (AI|Components|Blackboard|SetValueasBool _blackboard (Variables|BlackboardKeys|GetIsTouchingKey) true)))

(fn HasValidAttackTag
  (params (Actor :type Actor%20Object%20Reference))
  (for _array_element (Variables|PerceptibleTags|GetHostileList)
    (LocalVariables|SetHasTagLocal (or (Actor|ActorHasTag Actor _array_element) (LocalVariables|GetHasTagLocal))))
  (return (LocalVariables|GetHasTagLocal)))

(fn EndAttack
  (params (AttackTarget :type Actor%20Object%20Reference))
  (bind _tagisvalid (CallFunction|HasValidAttackTag AttackTarget))
  (if _tagisvalid
    (bind _returnvalue (Utilities|Set|Remove (Variables|Default|GetOverlappingTargets) AttackTarget))
    (if _returnvalue
      (if (Utilities|Set|IsEmpty (Variables|Default|GetOverlappingTargets))
        (AI|Components|Blackboard|SetValueasBool (Variables|Default|GetBlackboard) (Variables|BlackboardKeys|GetIsTouchingKey) false)
        (AI|Components|Blackboard|SetValueasObject (Variables|Default|GetBlackboard) (Variables|BlackboardKeys|GetEnemyActorKey) 0)
        (Class|AIPerceptionComponent|ForgetAll (Variables|Default|GetAIPerception))
        (else
          (bind _result (Utilities|Set|ToArray (Variables|Default|GetOverlappingTargets)))
          (AI|Components|Blackboard|SetValueasObject (Variables|Default|GetBlackboard) (Variables|BlackboardKeys|GetEnemyActorKey) (Utilities|Array|Get(acopy) _result)))))))