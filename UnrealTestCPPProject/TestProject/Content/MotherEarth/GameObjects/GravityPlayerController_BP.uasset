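; Player controller for RTS-style selection and command of minion units.
; Ctrl+left-click starts selection through the HUD and clears the current selection when the cursor trace hits nothing; releasing the mouse stops it.
; Helper functions maintain the selection list and each unit's selected state.
; Move, base and enemy orders write destination keys to each minion AI controller's blackboard, with enemy orders setting a target actor and move orders clearing it.
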(event Input|MouseEvents|LeftMouseButton
  (params (Key :type Key%20Structure))
  (bind _returnvalue (HUD|GetHUD))
  (:Pressed
    (if (Variables|Default|GetleftCtrlPressed)
      (Class|SelectionInterface|StartSelection(Message) _returnvalue)
      (if (not (.ReturnValue (Game|Player|GetHitResultUnderCursorbyChannel "TraceTypeQuery3" true)))
        (CallFunction|ClearUnitSelection))))
  (:Released
    (Class|SelectionInterface|StopSelection(Message) _returnvalue)))

(event Input|KeyboardEvents|LeftCtrl
  (params (Key :type Key%20Structure))
  (:Pressed
    (Variables|Default|SetleftCtrlPressed true))
  (:Released
    (Variables|Default|SetleftCtrlPressed false)))

(fn ConstructionScript
  (|CallParentFunction))

(fn ClearUnitSelection
  (bind _minionselection (Variables|Default|GetMinionSelection))
  (for _array_element _minionselection
    (Default|ISSelected _array_element false))
  (Utilities|Array|Clear _minionselection))

(fn AddUnittoSelection
  (params (MinionUnit :type Gravity%20Minion%20Character%20BP%20Object%20Reference))
  (Utilities|Array|AddUnique (Variables|Default|GetMinionSelection) MinionUnit)
  (Default|ISSelected MinionUnit true))

(fn RemoveUnitfromSelection
  (params (Minion%20Unit :type Gravity%20Minion%20Character%20BP%20Object%20Reference))
  (Utilities|Array|RemoveItem (Variables|Default|GetMinionSelection) Minion%20Unit)
  (Default|ISSelected Minion%20Unit false))

(fn MoveSelectedUnits
  (params (Location :type Vector))
  (for _array_element (Variables|Default|GetMinionSelection)
    (bind _asminion_aicontroller_planet_bp (Utilities|Casting|CastToMinionAIControllerPlanet_BP (AI|GetAIController _array_element)))
    (AI|Components|Blackboard|SetValueasVector (AI|GetBlackboard _asminion_aicontroller_planet_bp) (Variables|Default|GetMoveToDestKey) Location)
    (AI|Components|Blackboard|SetValueasBool (AI|GetBlackboard _asminion_aicontroller_planet_bp) (Variables|Default|GetTargetLocationSetKey) true)
    (AI|Components|Blackboard|SetValueasObject (AI|GetBlackboard _asminion_aicontroller_planet_bp) (Variables|Default|GetEnemyActorKey) 0)))

(fn SetBaseOfSelected
  (params (BaseActor :type Actor%20Object%20Reference))
  (bind _asbp_stone_henge_base (Utilities|Casting|CastToBP_StoneHengeBase BaseActor))
  (for _array_element (Variables|Default|GetMinionSelection)
    (bind _asminion_aicontroller_planet_bp (Utilities|Casting|CastToMinionAIControllerPlanet_BP (AI|GetAIController _array_element)))
    (AI|Components|Blackboard|SetValueasVector (AI|GetBlackboard _asminion_aicontroller_planet_bp) (Variables|Default|GetMoveToDestKey) (Transformation|GetActorLocation _asbp_stone_henge_base))
    (AI|Components|Blackboard|SetValueasBool (AI|GetBlackboard _asminion_aicontroller_planet_bp) (Variables|Default|GetTargetLocationSetKey) true)))

(fn SetEnemyOfSelected
  (params (EnemyActor :type Actor%20Object%20Reference))
  (bind _asgravity_enemy_character_bp (Utilities|Casting|CastToGravityEnemyCharacter_BP EnemyActor))
  (for _array_element (Variables|Default|GetMinionSelection)
    (bind _asminion_aicontroller_planet_bp (Utilities|Casting|CastToMinionAIControllerPlanet_BP (AI|GetAIController _array_element)))
    (AI|Components|Blackboard|SetValueasObject (Variables|/Script/AIModule.AIController|GetBlackboard _asminion_aicontroller_planet_bp) (Variables|Default|GetEnemyActorKey) _asgravity_enemy_character_bp)
    (AI|Components|Blackboard|SetValueasVector (Variables|/Script/AIModule.AIController|GetBlackboard _asminion_aicontroller_planet_bp) (Variables|Default|GetMoveToDestKey) (Transformation|GetActorLocation _asgravity_enemy_character_bp))
    (AI|Components|Blackboard|SetValueasBool (Variables|/Script/AIModule.AIController|GetBlackboard _asminion_aicontroller_planet_bp) (Variables|Default|GetTargetLocationSetKey) true)))