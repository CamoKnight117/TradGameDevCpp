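; BP_RegionBounds is a region volume that tracks which GravityEnemyCharacter_BP enemies are inside it.
; Shortly after BeginPlay it seeds an EnemyList set from the actors overlapping Bounds and prints their names, then begin and end overlap events add and remove enemies.
; GetRandomEnemy returns a random entry from that set, with its Success output wired to IsEmpty, so it is true when no enemies are present.
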(event EventBeginPlay
  (bind _bounds (Variables|Default|GetBounds))
  (bind _overlappingactors (Collision|GetOverlappingActors _bounds "/Game/MotherEarth/AI/Enemy/GravityEnemyCharacter_BP.GravityEnemyCharacter_BP_C" :!class /Script/Engine.PrimitiveComponent))
  (Utilities|FlowControl|Delay 0.1)
  (Utilities|Set|AddItems (Variables|Default|GetEnemyList) _overlappingactors)
  (for _array_element _overlappingactors
    (Development|PrintString (Utilities|GetDisplayName _array_element))))

(event Collision|EventActorBeginOverlap
  (params (OtherActor :type Actor%20Object%20Reference))
  (bind _asgravity_enemy_character_bp (Utilities|Casting|CastToGravityEnemyCharacter_BP OtherActor))
  (Utilities|Set|Add (Variables|Default|GetEnemyList) _asgravity_enemy_character_bp))

(event Collision|EventActorEndOverlap
  (params (OtherActor :type Actor%20Object%20Reference))
  (bind _asgravity_enemy_character_bp (Utilities|Casting|CastToGravityEnemyCharacter_BP OtherActor))
  (Utilities|Set|Remove (Variables|Default|GetEnemyList) _asgravity_enemy_character_bp))

(fn ConstructionScript)

(fn GetRandomEnemy
  (bind _result (Utilities|Set|ToArray (Variables|Default|GetEnemyList)))
  (return (.OutItem (Utilities|Array|Random _result)) (Utilities|Array|IsEmpty _result)))