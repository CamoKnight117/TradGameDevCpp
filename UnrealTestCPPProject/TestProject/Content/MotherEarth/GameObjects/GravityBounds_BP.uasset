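; Gravity volume actor that gives GravityPlayerCharacter_BP characters its own location as their gravity source via SetGravity.
; A non-looping timer runs the update once, half a second after BeginPlay.
; The update applies gravity to all characters passing IsInsideBounds, then again to those overlapping the Bounds sphere.
; IsInsideBounds compares unsquared distance against squared radius, so it reaches beyond larger spheres.
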(event Custom|updateGravity
  (CallFunction|SetPlayerGravity)
  (for _array_element (Collision|GetOverlappingActors (Variables|Default|GetBounds) 0 :!class /Script/Engine.PrimitiveComponent)
    (bind _asgravity_player_character_bp (Utilities|Casting|CastToGravityPlayerCharacter_BP _array_element))
    (Default|SetGravity _asgravity_player_character_bp (Transformation|GetActorLocation self))))

(event EventBeginPlay
  (Utilities|Time|SetTimerbyEvent (delegate Custom|updateGravity) 0.5))

(fn ConstructionScript)

(fn IsInsideBounds
  (params (Actor :type Actor%20Object%20Reference))
  (return (< (Math|Vector|Distance(Vector) (Transformation|GetActorLocation Actor) (Transformation|GetActorLocation)) (Math|Float|Square (Variables|/Script/Engine.SphereComponent|GetSphereRadius (Variables|Default|GetBounds))))))

(fn SetPlayerGravity
  (bind _outactors (Actor|GetAllActorsOfClass "/Game/MotherEarth/GravityPlayerCharacter_BP.GravityPlayerCharacter_BP_C"))
  (for _array_element _outactors
    (bind _isinsideboudns_ (CallFunction|IsInsideBounds _array_element))
    (if _isinsideboudns_
      (Default|SetGravity _array_element (Transformation|GetActorLocation)))))